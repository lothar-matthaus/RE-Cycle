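; BP_SpawnPoint is a spawn point actor that pairs itself with another spawn point in the level as its Destination.
; On BeginPlay, SetDestination gathers all BP_SpawnPoint actors and picks one at random, retrying whenever it picks itself.
; The retry has no exit condition, so a level with only one spawn point loops endlessly.
; Destination is only stored here, with no spawning or movement logic.
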(event `self.ReceiveBeginPlay`
  (`self.SetDestination`))

(fn `SetDestination`
  (bind _outactors (`GameplayStatics.GetAllActorsOfClass` "BP_SpawnPoint_C" :!label _label))
  (bind _output_get (set `self.Destination` (`|GetArrayItem` _outactors (`KismetMathLibrary.RandomIntegerInRange` 0 (- (`KismetArrayLibrary.Array_Length` _outactors) 1)))))
  (if (== _output_get self)
    (goto _label)))

(fn `UserConstructionScript`)