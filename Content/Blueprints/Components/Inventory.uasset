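; Weight-limited inventory component that stores collected waste as slots of item details and quantity.
; AddToInventory rejects waste that would push total weight over MaxWeight, otherwise Stack increments a same-named slot or AddItem appends a new one.
; TransferItens appends another inventory's slots that fit, without merging stacks, then removes from the source any slot matching one held here.
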(fn `Add Item`
  (params (itemQuantity :type Integer) (Waste :type "/Game/Blueprints/Actors/Waste/BP_Waste Object Reference"))
  (bind (_name _description _weight _producer _isrecyclable _price _type) (break `/Game/Blueprints/Structure/F_WasteDetail` (`/Game/Blueprints/Actors/Waste/BP_Waste.Details` Waste)))
  (`KismetArrayLibrary.Array_Add` (`self.Items`) (make `/Game/Blueprints/Structure/F_InventoryWasteSlot` (make `/Game/Blueprints/Structure/F_InventoryWaste` _name _description _weight _type _price) (`local.itemQuantity`)))
  (return))

(fn `AddItemToIndex`
  (params (Index :type Integer))
  (locals (WasStacked :type Boolean))
  (bind _output (`|GetArrayItem` (`self.Items`) Index))
  (setmembers `/Game/Blueprints/Structure/F_InventoryWasteSlot` :`StructRef` _output :`Quantity` (+ (`.Quantity_6_FA1AECF94C7A9BF2665BD29C520D526E` (break `/Game/Blueprints/Structure/F_InventoryWasteSlot` _output)) 1))
  (return))

(fn `AddToInventory`
  (params (Waste :type "/Game/Blueprints/Actors/Waste/BP_Waste Object Reference"))
  (returns (WasItemAdded :type Boolean))
  (locals (WasAdded :type Boolean :default false))
  (bind ((`Weight_6_CCA021244E9F8E30E0D2C282BDA939AC` _weight)) (break `/Game/Blueprints/Structure/F_WasteDetail` (`/Game/Blueprints/Actors/Waste/BP_Waste.Details` (`local.Waste`))))
  (bind _isinventoryempty (`self.IsInventoryEmpty`))
  (if _isinventoryempty
    (bind _canbeaddedtoinventory (`self.CanBeAddedToInventory` _weight))
    (if _canbeaddedtoinventory
      (`self.Add Item` 1 (`local.Waste`))
      (set `local.WasAdded` true)
      (else
        (set `local.WasAdded` false)))
    (else
      (bind _canbeaddedtoinventory_2 (`self.CanBeAddedToInventory` _weight))
      (if _canbeaddedtoinventory_2
        (bind _wasitemstacked (`self.Stack` (`local.Waste`)))
        (if _wasitemstacked
          (set `local.WasAdded` true)
          (else
            (`self.Add Item` 1 (`local.Waste`))
            (set `local.WasAdded` true)))
        (else
          (set `local.WasAdded` false)))))
  (return (`local.WasAdded`)))

(fn `CanBeAddedToInventory`
  (params (Weight :type "Float (double-precision)"))
  (returns (CanBeAddedToInventory :type Boolean))
  (locals (TotalInventoryWeight :type "Float (double-precision)") (CanBeAdded :type Boolean))
  (bind _totalinventoryweight (`local.TotalInventoryWeight`))
  (bind _returnvalue (> (+ _totalinventoryweight (`local.Weight`)) (`self.MaxWeight`)))
  (for _array_element (`self.Items`)
    (bind (_item _quantity) (break `/Game/Blueprints/Structure/F_InventoryWasteSlot` _array_element))
    (set `local.TotalInventoryWeight` (+ (* _quantity (`.Weight_22_32BD96614047E8E593F1F7B3D61F72B5` (break `/Game/Blueprints/Structure/F_InventoryWaste` _item))) _totalinventoryweight))
    (if _returnvalue
      (set `local.CanBeAdded` false)
      (break)
      (else
        (set `local.CanBeAdded` true))))
  (bind _output_get (set `local.CanBeAdded` (not _returnvalue)))
  (return _output_get))

(fn `IsInventoryEmpty`
  (returns (IsInventoryEmpty :type Boolean))
  (return (== (`KismetArrayLibrary.Array_Length` (`self.Items`)) 0)))

(fn `TransferItens`
  (params (FromInventory :type "/Game/Blueprints/Components/Inventory Object Reference (by ref)"))
  (locals (Item :type "/Game/Blueprints/Structure/F_InventoryWasteSlot Structure"))
  (bind _items (`/Game/Blueprints/Components/Inventory.Items` FromInventory))
  (for _array_element _items
    (set `local.Item` _array_element)
    (bind (_item _quantity) (break `/Game/Blueprints/Structure/F_InventoryWasteSlot` _array_element))
    (bind _canbeaddedtoinventory (`self.CanBeAddedToInventory` (* _quantity (`.Weight_22_32BD96614047E8E593F1F7B3D61F72B5` (break `/Game/Blueprints/Structure/F_InventoryWaste` _item)))))
    (if _canbeaddedtoinventory
      (`KismetArrayLibrary.Array_Add` (`self.Items`) (`local.Item`))))
  (for _array_element_2 (`self.Items`)
    (if (`KismetArrayLibrary.Array_Contains` _items _array_element_2)
      (`KismetArrayLibrary.Array_RemoveItem` _items _array_element_2)))
  (return))