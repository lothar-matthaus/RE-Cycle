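; BP_LevelDayTime is a level calendar that tracks day, day of week and year.
; A looping timer started on BeginPlay runs IncrementDay every two minutes, wrapping the weekday, updating its enum and rolling the year over when Day reaches 365.
; TakeTrashOut tells every BP_Resident to take out trash on two set weekdays, though nothing in this file calls it.
; GetCurrentDay exposes the day count.
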(event `self.ReceiveBeginPlay`
  (`KismetSystemLibrary.K2_SetTimer` null "IncrementDay" 120.0 true))

(fn `GetCurrentDay`
  (returns (Day :type Integer))
  (return (`self.Day`)))

(fn `IncrementDay`
  (bind _dayofweek (`self.DayOfWeek`))
  (`|ExecutionSequence`
    (:`then_0`
      (`/Engine/EditorBlueprintResources/StandardMacros.IncrementInt` (`self.Day`)
        (:`  `
          (`/Engine/EditorBlueprintResources/StandardMacros.IncrementInt` _dayofweek
            (:`  `
              (`|ExecutionSequence`
                (:`then_0`
                  (if (> _dayofweek 7)
                    (set `self.DayOfWeek` 1)))
                (:`then_1`
                  (set `self.DaysOfWeek` (cast `/Game/Blueprints/Enum/E_DayOfWeek` (`KismetMathLibrary.Conv_IntToByte` (- (`self.DayOfWeek`) 1)))))))))))
    (:`then_1`
      (if (== (`self.Day`) 365)
        (set `self.Day` 1)
        (`/Engine/EditorBlueprintResources/StandardMacros.IncrementInt` (`self.Year`))))))

(fn `TakeTrashOut`
  (bind _dayofweek (`self.DayOfWeek`))
  (if (or (== _dayofweek 2) (== _dayofweek 6))
    (bind _outactors (`GameplayStatics.GetAllActorsOfClass` "/Game/Blueprints/Characters/Resident/BP_Resident.BP_Resident_C"))
    (for _array_element _outactors
      (`/Game/Blueprints/Characters/Resident/BP_Resident.TakeTrashOut` _array_element))))

(fn `UserConstructionScript`)