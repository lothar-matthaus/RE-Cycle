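; Waste truck vehicle actor that drives along a randomly chosen spline path, then destroys itself.
; On BeginPlay it gets a random path and starts a timeline, slowed by a fixed play rate.
; Each update maps the timeline alpha to a distance along the spline and sets the truck's world location and rotation from that point.
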(event `self.ReceiveBeginPlay`
  (set `self.Path` (`/Game/Library/Functions/Game.GetRandomPath`))
  (`self.FollowPath`))

(event `FollowPath`
  (bind _spline (`/Game/Blueprints/Actors/Splines/BP_BasePathSpline.Spline` (`self.Path`)))
  (`TimelineComponent.SetPlayRate` (`self.FollowPathTimeLine`) (/ 1.0 50.0))
  (bind (_direction _followpath) (`Timeline|FollowPathTimeLine`)
    (:`Update`
      (bind _returnvalue (`KismetMathLibrary.Lerp` 0.0 (`SplineComponent.GetSplineLength` _spline) _followpath))
      (`self.K2_SetActorTransform` (`KismetMathLibrary.MakeTransform` (`SplineComponent.GetLocationAtDistanceAlongSpline` _spline _returnvalue "World") (`SplineComponent.GetRotationAtDistanceAlongSpline` _spline _returnvalue "World"))))
    (:`Finished`
      (`self.K2_DestroyActor`))))

(fn `UserConstructionScript`)