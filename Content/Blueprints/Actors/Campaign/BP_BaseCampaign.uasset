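; BP_BaseCampaign is a timed campaign actor that gradually raises the conscience of residents.
; On BeginPlay it loads its service row from DT_Services, caches all BP_Resident actors and shows a notification widget.
; A looping one-second timer adds a small random conscience gain to each resident and counts down the duration, then closes the notification and destroys the actor.
; BP_GameState's overall info is updated at start and destruction, tracking active social media campaigns.
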(event `self.ReceiveBeginPlay`
  (`self.SetCampaign` (`self.ServiceName`))
  (bind _asbp_game_state (cast `/Game/Blueprints/Game/BP_GameState` (`GameplayStatics.GetGameState`)))
  (set `self.Game State` _asbp_game_state)
  (bind _outactors (`GameplayStatics.GetAllActorsOfClass` "/Game/Blueprints/Characters/Resident/BP_Resident.BP_Resident_C"))
  (set `self.PersonList` _outactors)
  (`self.CreateCampaignNotificationWidget`)
  (`/Game/Blueprints/Game/BP_GameState.UpdateOverallInfo` (`self.Game State`) (make `/Game/Blueprints/Structure/F_OverallInfo` :`TotalRunnedCampaigns` 1))
  (set `self.LifeSpan` (`.Duration_11_F3B0E8F94D2078569F9CE5B3D227ED6E` (break `/Game/Blueprints/Structure/F_Service` (`self.Service`))))
  (`KismetSystemLibrary.K2_SetTimer` null "UpdatePersonConscience" 1.0 true))

(event `self.ReceiveDestroyed`
  (`/Game/Blueprints/Game/BP_GameState.UpdateOverallInfo` (`self.Game State`) (make `/Game/Blueprints/Structure/F_OverallInfo` :`TotalActiveSocialMediaCampaign` -1)))

(fn `CreateCampaignNotificationWidget`
  (bind ((`Name_5_477EC45E49E6C086383319AD1A5CEDAE` _name) (`Duration_11_F3B0E8F94D2078569F9CE5B3D227ED6E` _duration)) (break `/Game/Blueprints/Structure/F_Service` (`self.Service`)))
  (bind _returnvalue (`|CreateWidget` "/Game/Blueprints/UI/Sevices/WBP_CampaignNotification.WBP_CampaignNotification_C"))
  (bind _output_get (set `self.CampaignNotification` _returnvalue))
  (`/Game/Blueprints/UI/Sevices/WBP_CampaignNotification.SetCampaingMessage` _output_get (`|FormatText` "CampaignMessage" _name _duration) _duration)
  (`UserWidget.AddToViewport` _output_get 0))

(fn `SetCampaign`
  (params (ServiceName :type Name))
  (bind _returnvalue (`|GetDataTableRow` "/Game/Blueprints/DataTable/DT_Services.DT_Services" ServiceName)
    (:`then`
      (set `self.Service` _returnvalue))))

(fn `UpdatePersonConscience`
  (`|ExecutionSequence`
    (:`then_0`
      (for _array_element (`self.PersonList`)
        (`/Game/Blueprints/Characters/Person/BP_BasePerson.IncrementConscience` _array_element (`KismetMathLibrary.RandomFloatInRange` 0.0001 0.001))))
    (:`then_1`
      (bind _result (`/Engine/EditorBlueprintResources/StandardMacros.DecrementFloat` (`self.LifeSpan`))
        (:`  `
          (if (<= _result 0.0)
            (`/Game/Blueprints/UI/Sevices/WBP_CampaignNotification.CloseNotification` (`self.CampaignNotification`))
            (`self.K2_DestroyActor`)))))))

(fn `UserConstructionScript`)