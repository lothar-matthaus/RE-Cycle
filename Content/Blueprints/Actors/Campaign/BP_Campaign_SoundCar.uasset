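; Campaign sound car actor that travels along a spline path as part of a campaign service.
; On BeginPlay it picks a random path, teleports to it and registers itself in the GameState's overall campaign counts.
; A timeline, rate-scaled by the inverse of the service duration, sets the car's location and rotation from distance along the spline.
; On destruction it sends a negative update to the overall info.
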(event `self.ReceiveBeginPlay`
  (`parent.ReceiveBeginPlay`)
  (bind _output_get (set `self.Path` (`/Game/Library/Functions/Game.GetRandomPath`)))
  (`self.K2_SetActorLocation` (`self.K2_GetActorLocation` _output_get) false true)
  (`/Game/Blueprints/Game/BP_GameState.UpdateOverallInfo` (`self.Game State`) (make `/Game/Blueprints/Structure/F_OverallInfo` :`TotalSoundCarCampaign` 1 :`TotalActiveSoundCarCampaign` 1))
  (`self.FollowPath`))

(event `self.ReceiveDestroyed`
  (`/Game/Blueprints/Game/BP_GameState.UpdateOverallInfo` (`self.Game State`) (make `/Game/Blueprints/Structure/F_OverallInfo` :`TotalActiveSoundCarCampaign` -1)))

(event `FollowPath`
  (bind _spline (`/Game/Blueprints/Actors/Splines/BP_BasePathSpline.Spline` (`self.Path`)))
  (`TimelineComponent.SetPlayRate` (`self.FollowPathTimeLine`) (/ 1.0 (`.Duration_11_F3B0E8F94D2078569F9CE5B3D227ED6E` (break `/Game/Blueprints/Structure/F_Service` (`self.Service`)))))
  (bind (_direction _followpath) (`Timeline|FollowPathTimeLine`)
    (:`Update`
      (bind _returnvalue (`KismetMathLibrary.Lerp` 0.0 (`SplineComponent.GetSplineLength` _spline) _followpath))
      (`self.K2_SetActorTransform` (`KismetMathLibrary.MakeTransform` (`SplineComponent.GetLocationAtDistanceAlongSpline` _spline _returnvalue "World") (`SplineComponent.GetRotationAtDistanceAlongSpline` _spline _returnvalue "World"))))))

(fn `UserConstructionScript`
  (`parent.UserConstructionScript`))