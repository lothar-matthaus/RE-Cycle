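; Base house actor for a waste-management game: a residence that spawns residents and tracks their waste.
; BeginPlay sets resident count by house size, assigns a random number, spawns residents on nearby navmesh and updates the GameState.
; It tallies waste by type, averages resident mood and conscience, and exchanges inventory items.
; Interaction opens an info widget unless another house shows one; door overlaps play sounds and toggle resident visibility.
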(event `self.ReceiveBeginPlay`
  ;[1 1 1] BeginPlay
  (`|ExecutionSequence`
    (:`then_0`
      (switch `/Game/Blueprints/Enum/E_HouseSize` (`.Size_9_A9DC899A409286DCAA4138B621EB3EB3` (break `/Game/Blueprints/Structure/F_HouseDetail` (`self.Details`)))
        (:`NewEnumerator0`
          (set `self.NumberOfResidents` 4))
        (:`NewEnumerator1`
          (set `self.NumberOfResidents` 6))
        (:`NewEnumerator2`
          (set `self.NumberOfResidents` 8))))
    (:`then_1`
      (`self.SetHouseDetails`)
      (`self.CreateFamily`)
      (bind _asbp_game_state (cast `/Game/Blueprints/Game/BP_GameState` (`GameplayStatics.GetGameState`)))
      (set `self.GameState` _asbp_game_state)
      (`/Game/Blueprints/Game/BP_GameState.UpdateOverallInfo` (`self.GameState`) (make `/Game/Blueprints/Structure/F_OverallInfo` :`NumberOfFamilies` 1)))))

(event `/Game/Blueprints/Interfaces/BI_Interactable.Interact`
  (params (Interactor :type "Actor Object Reference (by ref)"))
  (bind _houseinfo (`self.HouseInfo`))
  ;[1 1 1] Create Widget
  (if (and (not (`SceneComponent.IsVisible` _houseinfo)) (`self.CheckOpenedWidgets`))
    (bind _returnvalue (`|CreateWidget` "/Game/Blueprints/UI/House/WBP_HouseInfo.WBP_HouseInfo_C"))
    (`/Game/Blueprints/UI/House/WBP_HouseInfo.SetResidence` _returnvalue self)
    (`WidgetComponent.SetWidget` _houseinfo _returnvalue)
    (`SceneComponent.SetVisibility` _houseinfo true true)
    (`GameplayStatics.PlaySoundAtLocation` "/Game/Audio/SFX/House/Bell/AU_DoorBell.AU_DoorBell" (`self.K2_GetActorLocation`) (struct) 0.8 1.0 0.0 "/Game/Audio/Attenuation/AU_Vehicle_Attenuation.AU_Vehicle_Attenuation" null null null)))

(event `/Game/Blueprints/Interfaces/BI_Widget.UpdateWidget`
  (bind _returnvalue (`WidgetComponent.GetUserWidgetObject` (`self.HouseInfo`)))
  (bind _aswbp_house_info (cast `/Game/Blueprints/UI/House/WBP_HouseInfo` _returnvalue :!pure true))
  ;[1 1 1] Update Widgeet
  (`/Engine/EditorBlueprintResources/StandardMacros.IsValid` _returnvalue
    (:`Is Valid`
      (`/Game/Blueprints/UI/House/WBP_HouseInfo.UpdateHouseDetails` _aswbp_house_info)
      (`/Game/Blueprints/UI/House/WBP_HouseInfo.UpdateHouseInventory` _aswbp_house_info)
      (`/Game/Blueprints/UI/House/WBP_HouseInfo.UpdateHouseStats` _aswbp_house_info))))

(event `self.Mesh.OnBeginCursorOver`
  (params (TouchedComponent :type "PrimitiveComponent Object Reference"))
  ;[1 1 1] Change Mouse Cursor
  (set `PlayerController.CurrentMouseCursor` "Hand" (`GameplayStatics.GetPlayerController` 0)))

(event `self.Mesh.OnEndCursorOver`
  (params (TouchedComponent :type "PrimitiveComponent Object Reference"))
  ;[1 1 1] Change Mouse Cursor
  (set `PlayerController.CurrentMouseCursor` "Default" (`GameplayStatics.GetPlayerController` 0)))

(event `self.BackDoorCollision.OnComponentBeginOverlap`
  (params (OverlappedComponent :type "PrimitiveComponent Object Reference") (OtherActor :type "Actor Object Reference") (OtherComp :type "PrimitiveComponent Object Reference") (OtherBodyIndex :type Integer) (bFromSweep :type Boolean) (SweepResult :type "HitResult Structure (by ref)"))
  ;[1 1 1] Play door Sound
  (bind _asbp_resident (cast `/Game/Blueprints/Characters/Resident/BP_Resident` OtherActor))
  (`GameplayStatics.PlaySoundAtLocation` "/Game/Audio/SFX/House/Door/Door.Door" (`self.K2_GetActorLocation`) (struct) 1.0 1.0 0.0 "/Game/Audio/Attenuation/AU_Door_Attenuation.AU_Door_Attenuation" null null null)
  (if (`/Game/Blueprints/Characters/Person/BP_BasePerson.bIsAtHome` _asbp_resident)
    (bind _mesh (`Character.Mesh` _asbp_resident))
    (`SceneComponent.SetVisibility` _mesh false true)
    (else
      (`SceneComponent.SetVisibility` _mesh true true))))

(event `self.FrontDoorCollision.OnComponentBeginOverlap`
  (params (OverlappedComponent :type "PrimitiveComponent Object Reference") (OtherActor :type "Actor Object Reference") (OtherComp :type "PrimitiveComponent Object Reference") (OtherBodyIndex :type Integer) (bFromSweep :type Boolean) (SweepResult :type "HitResult Structure (by ref)"))
  ;[1 1 1] Play door Sound
  (bind _asbp_resident (cast `/Game/Blueprints/Characters/Resident/BP_Resident` OtherActor))
  (`GameplayStatics.PlaySoundAtLocation` "/Game/Audio/SFX/House/Door/Door.Door" (`self.K2_GetActorLocation` OtherActor) (struct) 1.0 1.0 0.0 "/Game/Audio/Attenuation/AU_Door_Attenuation.AU_Door_Attenuation" null null null)
  (if (`/Game/Blueprints/Characters/Person/BP_BasePerson.bIsAtHome` _asbp_resident)
    (bind _mesh (`Character.Mesh` _asbp_resident))
    (`SceneComponent.SetVisibility` _mesh false false)
    (else
      (`SceneComponent.SetVisibility` _mesh true false))))

(fn `CheckOpenedWidgets`
  (returns (CanOpenWidget :type Boolean))
  (locals (bCanOpenWidget :type Boolean :default true))
  (bind _outactors (`GameplayStatics.GetAllActorsOfClass` "BP_BaseHouse_C"))
  (for _array_element _outactors
    (if (`SceneComponent.IsVisible` (`/Game/Blueprints/Actors/House/BP_BaseHouse.HouseInfo` _array_element))
      (set `local.bCanOpenWidget` false)
      (break)))
  (return (`local.bCanOpenWidget`)))

(fn `CreateFamily`
  (locals (Resident :type "/Game/Blueprints/Characters/Resident/BP_Resident Object Reference") (SpawnPointTransform :type "Transform Structure") (SpawnList :type "Array of /Game/Blueprints/Components/Spawn/BP_SpawnPoint Object Reference"))
  (for _ (range 1 (+ (`self.NumberOfResidents`) 1))
    (bind _randomlocation (`NavigationSystemV1.K2_GetRandomLocationInNavigableRadius` (`self.K2_GetActorLocation` self) (`KismetMathLibrary.RandomFloatInRange` 500.0 800.0) null null))
    (bind _returnvalue (`|SpawnActorFromClass` "/Game/Blueprints/Characters/Resident/BP_Resident.BP_Resident_C" (`KismetMathLibrary.MakeTransform` (+ _randomlocation (0.0 0.0 100.0))) "AdjustIfPossibleButAlwaysSpawn" "OverrideRootScale" self (`self.Instigator`)))
    (set `local.Resident` _returnvalue)
    (`KismetArrayLibrary.Array_Add` (`.Residents_13_7C265B8C45FC7A4D17ABEDB629AB7EA5` (break `/Game/Blueprints/Structure/F_HouseDetail` (`self.Details`))) (`local.Resident`))
    (setmembers `/Game/Blueprints/Structure/F_PersonDetail` :`StructRef` (`/Game/Blueprints/Characters/Person/BP_BasePerson.Details` (`local.Resident`)) :`Residence` self)))

(fn `GetAverageConscience`
  (returns (Conscience :type "Float (double-precision)"))
  (locals (AverageConscience :type "Float (double-precision)") (TotalConscience :type "Float (double-precision)"))
  (bind (_number _size _residents) (break `/Game/Blueprints/Structure/F_HouseDetail` (`self.Details`)))
  (for _array_element _residents
    (set `local.TotalConscience` (+ (`.Conscience_35_519E32E14799A62A65B328B0DD622DAE` (break `/Game/Blueprints/Structure/F_PersonDetail` (`/Game/Blueprints/Characters/Person/BP_BasePerson.Details` _array_element))) (`local.TotalConscience`))))
  (bind _output_get (set `local.AverageConscience` (/ (`local.TotalConscience`) (`KismetArrayLibrary.Array_Length` _residents))))
  (return _output_get))

(fn `GetAverageMood`
  (returns (Mood :type "Float (double-precision)"))
  (locals (TotalMood :type "Float (double-precision)") (AverageMood :type "Float (double-precision)"))
  (bind (_number _size _residents) (break `/Game/Blueprints/Structure/F_HouseDetail` (`self.Details`)))
  (`|ExecutionSequence`
    (:`then_0`
      (for _array_element _residents
        (set `local.TotalMood` (+ (`.Mood_36_7BCD7D5140C9C277061647BB3AC58066` (break `/Game/Blueprints/Structure/F_PersonDetail` (`/Game/Blueprints/Characters/Person/BP_BasePerson.Details` _array_element))) (`local.TotalMood`))))
      (set `local.AverageMood` (/ (`local.TotalMood`) (`KismetArrayLibrary.Array_Length` _residents))))
    (:`then_1`
      (return (`local.AverageMood`)))))

(fn `RemoveWidget`
  (bind _houseinfo (`self.HouseInfo`))
  (`WidgetComponent.SetWidget` _houseinfo null)
  (`SceneComponent.SetVisibility` _houseinfo false true))

(fn `SetHouseDetails`
  (setmembers `/Game/Blueprints/Structure/F_HouseDetail` :`StructRef` (`self.Details`) :`Number` (`KismetMathLibrary.RandomInteger` 1000)))

(fn `TransferItemsFromInventory`
  (params (Iterator :type "Actor Object Reference"))
  (returns (HasFinishedTransfer :type Boolean))
  (locals (Person :type "/Game/Blueprints/Characters/Person/BP_BasePerson Object Reference"))
  (bind _asbp_base_person (cast `/Game/Blueprints/Characters/Person/BP_BasePerson` Iterator))
  (bind _output_get (set `local.Person` _asbp_base_person))
  (`|ExecutionSequence`
    (:`then_0`
      (`/Game/Blueprints/Components/Inventory.TransferItemsFromInventory` (`self.Inventory`) (`/Game/Blueprints/Characters/Person/BP_BasePerson.Inventory` _output_get)))
    (:`then_1`
      (return true))))

(fn `TransferItemsFromTrashBin`
  (params (Iterator :type "Actor Object Reference (by ref)"))
  (returns (HasFinishedTransfering :type Boolean))
  (return false))

(fn `UpdateHouseStats`
  (params (Waste :type "/Game/Blueprints/Actors/Waste/BP_Waste Object Reference"))
  (bind _stats (`self.Stats`))
  (bind _stats_2 (`self.Stats`))
  (bind _stats_3 (`self.Stats`))
  (bind ((`TotalOrganicWasteWeight_55_CD97D9E1488499C669AE47BA1609289A` _totalorganicwasteweight) (`TotalWeightGenerated_62_D278A50F44EDFB5F8BA78A9C3AC53A69` _totalweightgenerated)) (break `/Game/Blueprints/Structure/F_Stats` _stats))
  (bind ((`TotalWasteWeigh_57_BE5538EF4582794FEDE90095D7763206` _totalwasteweigh) (`TotalWeightGenerated_62_D278A50F44EDFB5F8BA78A9C3AC53A69` _totalweightgenerated_2)) (break `/Game/Blueprints/Structure/F_Stats` _stats_2))
  (bind ((`TotalRecyclableWasteWeight_56_BE899F404B2463B50D1250AE1D050569` _totalrecyclablewasteweight) (`TotalRecyclablePrice_59_54B91AE04B89188609D6DD9B937430ED` _totalrecyclableprice) (`TotalWeightGenerated_62_D278A50F44EDFB5F8BA78A9C3AC53A69` _totalweightgenerated_3)) (break `/Game/Blueprints/Structure/F_Stats` _stats_3))
  (bind ((`Name_34_90C7E46B4048F4C6621C8F87493905A4` _name) (`Description_35_FA3A56E8438BCBBAD3D3F19E2BF0C5A9` _description) (`Weight_6_CCA021244E9F8E30E0D2C282BDA939AC` _weight) (`Price_18_2B5D253C42D90CED3CEA0485A9C32E50` _price) (`Type_12_E4B9AF6E4BFB737C2F9D1DA63FAC2614` _type)) (break `/Game/Blueprints/Structure/F_WasteDetail` (`/Game/Blueprints/Actors/Waste/BP_Waste.Details` (`local.Waste`))))
  (if (`KismetSystemLibrary.IsValid` Waste)
    (switch `/Game/Blueprints/Enum/E_WasteType` _type
      (:`NewEnumerator0`
        ;[1 1 1] Organic Waste Stats
        (setmembers `/Game/Blueprints/Structure/F_Stats` :`StructRef` _stats :`TotalOrganicWasteWeight` (+ _totalorganicwasteweight _weight) :`TotalWeightGenerated` (+ _totalweightgenerated _weight)))
      (:`NewEnumerator1`
        ;[1 1 1] Recyclable Waste Stats
        (setmembers `/Game/Blueprints/Structure/F_Stats` :`StructRef` _stats_3 :`TotalRecyclableWasteWeight` (+ _totalrecyclablewasteweight _weight) :`TotalRecyclablePrice` (+ _totalrecyclableprice _price) :`TotalWeightGenerated` (+ _totalweightgenerated_3 _weight) :!label _label))
      (:`NewEnumerator2`
        (goto _label))
      (:`NewEnumerator3`
        (goto _label))
      (:`NewEnumerator4`
        (goto _label))
      (:`NewEnumerator7`
        (goto _label))
      (:`NewEnumerator8`
        ;[1 1 1] Waste Stats
        (setmembers `/Game/Blueprints/Structure/F_Stats` :`StructRef` _stats_2 :`TotalWasteWeigh` (+ _totalwasteweigh _weight) :`TotalWeightGenerated` (+ _totalweightgenerated_2 _weight))))))

(fn `UpdateOverallInfo`)

(fn `UserConstructionScript`)