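; BP_SpawnPedestrian is a level spawner actor that periodically populates the level with pedestrians.
; On BeginPlay it starts a looping timer whose interval is randomized once, calling SpawnPedestrian to spawn a BP_Pedestrian at a random BP_SpawnPoint, adjusting for collision but always spawning.
; A second looping timer targets IncrementDay by name, but no such function appears in this Blueprint.
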(event `self.ReceiveBeginPlay`
  (`KismetSystemLibrary.PrintString` "Hello")
  (`KismetSystemLibrary.K2_SetTimer` null "SpawnPedestrian" (`KismetMathLibrary.RandomFloatInRange` 1.0 5.0) true)
  (`KismetSystemLibrary.K2_SetTimer` null "IncrementDay" 3.0 true))

(fn `SpawnPedestrian`
  (bind _outactors (`GameplayStatics.GetAllActorsOfClass` "/Game/Blueprints/Actors/Spawn/BP_SpawnPoint.BP_SpawnPoint_C"))
  (bind _returnvalue (`KismetArrayLibrary.Array_Length` _outactors))
  (if (not (== _returnvalue 0))
    (`|SpawnActorFromClass` "/Game/Blueprints/Characters/Pedestrian/BP_Pedestrian.BP_Pedestrian_C" (`self.GetTransform` (`|GetArrayItem` _outactors (`KismetMathLibrary.RandomIntegerInRange` 0 (- _returnvalue 1)))) "AdjustIfPossibleButAlwaysSpawn" "OverrideRootScale" null null)))

(fn `UserConstructionScript`)