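; BP_Composter is a bin actor that turns stored waste of one producer type into fertilizer.
; A looping timer takes one unit per matching inventory slot, accumulating weight until the required amount starts production and marking emptied slots for removal.
; A second timer advances progress, then spawns a BP_Waste with the DT_Waste Fertilizer row, adds it to the inventory and refreshes the widget.
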(event `self.ReceiveBeginPlay`
  (`parent.ReceiveBeginPlay`)
  (`KismetSystemLibrary.K2_SetTimer` null "CanGenerateFertilizer" 1.0 true))

(fn `CanGenerateFertilizer`
  (locals (WasteList :type "Array of Integer"))
  (bind _items (`/Game/Blueprints/Components/Inventory.Items` (`self.Inventory`)))
  (if (not (`self.bCanGenerateFertilizer`))
    (`|ExecutionSequence`
      (:`then_0`
        (for (_array_element _array_index) _items
          (bind (_item _quantity) (break `/Game/Blueprints/Structure/F_InventoryWasteSlot` _array_element))
          (bind ((`Weight_6_CCA021244E9F8E30E0D2C282BDA939AC` _weight) (`Producer_28_8C142CCC414944C4234991AB135A7363` _producer)) (break `/Game/Blueprints/Structure/F_WasteDetail` _item))
          (if (`|EnumEquality` _producer "NewEnumerator0")
            (bind _structout (setmembers `/Game/Blueprints/Structure/F_InventoryWasteSlot` :`StructRef` _array_element :`Quantity` (`KismetMathLibrary.Clamp` (- _quantity 1) 0 _quantity)))
            (`KismetArrayLibrary.Array_Set` (`/Game/Blueprints/Components/Inventory.Items` (`self.Inventory`)) _array_index _structout)
            (if (<= _quantity 0)
              (`KismetArrayLibrary.Array_Add` (`local.WasteList`) _array_index))
            (bind _output_get (set `self.TotalWasteWeights` (+ _weight (`self.TotalWasteWeights`))))
            (if (>= _output_get (`self.RequiredWeightToGenerateFertilizer`))
              (set `self.bCanGenerateFertilizer` true)
              (set `self.TotalWasteWeights` 0.0)
              (break))))
        (`/Game/Blueprints/Interfaces/BI_Widget.UpdateWidget`))
      (:`then_1`
        (for _array_element_2 (`local.WasteList`)
          (`KismetArrayLibrary.Array_Remove` _items _array_element_2))
        (if (`self.bCanGenerateFertilizer`)
          (`KismetSystemLibrary.K2_SetTimer` null "GenerateFertilizer" 1.0 true)
          (`/Game/Blueprints/Interfaces/BI_Widget.UpdateWidget`))))))

(fn `GenerateFertilizer`
  (locals (Fertilizer :type "/Game/Blueprints/Structure/F_WasteDetail Structure"))
  (if (`self.bCanGenerateFertilizer`)
    (bind _result (`/Engine/EditorBlueprintResources/StandardMacros.IncrementFloat` (`self.FertilizerProgress`))
      (:`  `
        (if (== _result (`self.TimeToGenerateFertilizer`))
          (set `self.FertilizerProgress` 0.0)
          (set `self.bCanGenerateFertilizer` false)
          (bind _returnvalue (`|GetDataTableRow` "/Game/Blueprints/DataTable/DT_Waste.DT_Waste" "Fertilizer")
            (:`then`
              (bind _output_get (set `local.Fertilizer` _returnvalue))
              (bind _returnvalue_2 (`|SpawnActorFromClass` "/Game/Blueprints/Actors/Waste/BP_Waste.BP_Waste_C" (`self.GetTransform`) "Undefined" "OverrideRootScale" null null))
              (set `/Game/Blueprints/Actors/Waste/BP_Waste.Details` _output_get _returnvalue_2)
              (`/Game/Blueprints/Components/Inventory.AddToInventory` (`self.Inventory`) _returnvalue_2)
              (`/Game/Blueprints/Interfaces/BI_Widget.UpdateWidget`))))))))

(fn `UserConstructionScript`
  (`parent.UserConstructionScript`))