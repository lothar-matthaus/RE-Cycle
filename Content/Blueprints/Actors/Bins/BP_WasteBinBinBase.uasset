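; Base waste bin actor, typed as composter, recyclable or waste, that exchanges inventory items with BP_BasePerson and opens an info widget on interaction.
; Deposits are filtered by item type, except that waste bins accept any item when the person fails a random Conscience roll.
; People can also take filtered items back out.
; A one-second timer drains durability, then destroys the bin if empty or caps its capacity at current weight.
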(event `self.ReceiveBeginPlay`
  (bind _inventory (`self.Inventory`))
  (switch `/Game/Blueprints/Enum/E_BinType` (`self.Type`)
    (:`NewEnumerator0`
      (set `/Game/Blueprints/Components/Inventory.Name` "OrganicWasteBin" _inventory))
    (:`NewEnumerator1`
      (set `/Game/Blueprints/Components/Inventory.Name` "RecyclableWasteBin" _inventory))
    (:`NewEnumerator3`
      (set `/Game/Blueprints/Components/Inventory.Name` "WasteBin" _inventory)))
  (set `self.MaxDurability` (`self.Durability`))
  (`KismetSystemLibrary.K2_SetTimer` null "DecreaseDurability" 1.0 true))

(event `self.StaticMesh.OnBeginCursorOver`
  (params (TouchedComponent :type "PrimitiveComponent Object Reference"))
  ;[1 1 1] Set Default Cursor
  (set `PlayerController.CurrentMouseCursor` "Hand" (`GameplayStatics.GetPlayerController` 0)))

(event `self.StaticMesh.OnEndCursorOver`
  (params (TouchedComponent :type "PrimitiveComponent Object Reference"))
  ;[1 1 1] Set Default Cursor
  (set `PlayerController.CurrentMouseCursor` "Default" (`GameplayStatics.GetPlayerController` 0)))

(event `/Game/Blueprints/Interfaces/BI_Interactable.Interact`
  (params (Interactor :type "Actor Object Reference (by ref)"))
  ;[1 1 1] Comment
  (bind _returnvalue (`|CreateWidget` "/Game/Blueprints/UI/TrashBin/WBP_Trash_Info.WBP_Trash_Info_C" (`GameplayStatics.GetPlayerController` 0)))
  (bind _output_get (set `self.TrashBinInfoWidget` _returnvalue))
  (`/Game/Blueprints/UI/TrashBin/WBP_Trash_Info.SetWasteBin` _output_get self)
  (`UserWidget.AddToViewport` _output_get 0))

(event `self.UpdateWidget`
  (bind _trashbininfowidget (`self.TrashBinInfoWidget`))
  ;[1 1 1] Update Widget if Opened
  (`/Engine/EditorBlueprintResources/StandardMacros.IsValid` _trashbininfowidget
    (:`Is Valid`
      (`/Game/Blueprints/UI/TrashBin/WBP_Trash_Info.UpdateTrashBinInventory` _trashbininfowidget))))

(fn `DecreaseDurability`
  (bind _inventory (`self.Inventory`))
  (bind _result (`/Engine/EditorBlueprintResources/StandardMacros.DecrementFloat` (`self.Durability`))
    (:`  `
      (if (<= _result 0.0)
        (bind _isinventoryempty (`/Game/Blueprints/Components/Inventory.IsInventoryEmpty` (`self.Inventory`)))
        (if _isinventoryempty
          (`self.K2_DestroyActor`)
          (else
            (set `/Game/Blueprints/Components/Inventory.MaxWeight` (`/Game/Blueprints/Components/Inventory.Total Weight` _inventory) _inventory)))))))

(fn `TransferItemsFromInventory`
  (params (Iterator :type "Actor Object Reference"))
  (returns (HasFinishedTransfer :type Boolean))
  (bind _personreference (`self.PersonReference`))
  (bind _items (`/Game/Blueprints/Components/Inventory.Items` (`/Game/Blueprints/Characters/Person/BP_BasePerson.Inventory` _personreference)))
  (bind _asbp_base_person (cast `/Game/Blueprints/Characters/Person/BP_BasePerson` Iterator))
  (set `self.PersonReference` _asbp_base_person)
  (`|ExecutionSequence`
    (:`then_0`
      (switch `/Game/Blueprints/Enum/E_BinType` (`self.Type`)
        (:`NewEnumerator0`
          (for _array_element (`/Game/Blueprints/Components/Inventory.Items` (`/Game/Blueprints/Characters/Person/BP_BasePerson.Inventory` (`self.PersonReference`)))
            (if (`|EnumEquality` (`.Type_12_E4B9AF6E4BFB737C2F9D1DA63FAC2614` (break `/Game/Blueprints/Structure/F_WasteDetail` (`.Item_7_4E992E384499524884C00BA60CBAADB4` (break `/Game/Blueprints/Structure/F_InventoryWasteSlot` _array_element)))) "NewEnumerator0")
              (bind _wasadded (`/Game/Blueprints/Components/Inventory.TransferItem` (`self.Inventory`) _array_element))
              (if _wasadded
                (`KismetArrayLibrary.Array_RemoveItem` (`/Game/Blueprints/Components/Inventory.Items` (`/Game/Blueprints/Characters/Person/BP_BasePerson.Inventory` (`self.PersonReference`))) _array_element)))))
        (:`NewEnumerator1`
          (for _array_element_2 _items
            (bind ((`Name_34_90C7E46B4048F4C6621C8F87493905A4` _name) (`Description_35_FA3A56E8438BCBBAD3D3F19E2BF0C5A9` _description) (`Type_12_E4B9AF6E4BFB737C2F9D1DA63FAC2614` _type)) (break `/Game/Blueprints/Structure/F_WasteDetail` (`.Item_7_4E992E384499524884C00BA60CBAADB4` (break `/Game/Blueprints/Structure/F_InventoryWasteSlot` _array_element_2))))
            (if (and (`|EnumInequality` _type "NewEnumerator0") (`|EnumInequality` _type "NewEnumerator8"))
              (bind _wasadded_2 (`/Game/Blueprints/Components/Inventory.TransferItem` (`self.Inventory`) _array_element_2))
              (if _wasadded_2
                (`KismetArrayLibrary.Array_RemoveItem` (`/Game/Blueprints/Components/Inventory.Items` (`/Game/Blueprints/Characters/Person/BP_BasePerson.Inventory` (`self.PersonReference`))) _array_element_2)))))
        (:`NewEnumerator3`
          (if (>= (`.Conscience_35_519E32E14799A62A65B328B0DD622DAE` (break `/Game/Blueprints/Structure/F_PersonDetail` (`/Game/Blueprints/Characters/Person/BP_BasePerson.Details` _personreference))) (`KismetMathLibrary.RandomFloatInRange` 0.0 100.0))
            (for _array_element_3 _items
              (if (`|EnumEquality` (`.Type_12_E4B9AF6E4BFB737C2F9D1DA63FAC2614` (break `/Game/Blueprints/Structure/F_WasteDetail` (`.Item_7_4E992E384499524884C00BA60CBAADB4` (break `/Game/Blueprints/Structure/F_InventoryWasteSlot` _array_element_3)))) "NewEnumerator8")
                (bind _wasadded_3 (`/Game/Blueprints/Components/Inventory.TransferItem` (`self.Inventory`) _array_element_3))
                (if _wasadded_3
                  (`KismetArrayLibrary.Array_RemoveItem` (`/Game/Blueprints/Components/Inventory.Items` (`/Game/Blueprints/Characters/Person/BP_BasePerson.Inventory` (`self.PersonReference`))) _array_element_3))))
            (else
              (for _array_element_4 (`/Game/Blueprints/Components/Inventory.Items` (`/Game/Blueprints/Characters/Person/BP_BasePerson.Inventory` (`self.PersonReference`)))
                (bind _wasadded_4 (`/Game/Blueprints/Components/Inventory.TransferItem` (`self.Inventory`) _array_element_4))
                (if _wasadded_4
                  (`KismetArrayLibrary.Array_RemoveItem` _items _array_element_4))))))))
    (:`then_1`
      (return true))))

(fn `TransferItemsFromTrashBin`
  (params (Iterator :type "Actor Object Reference (by ref)"))
  (returns (HasFinishedTransfering :type Boolean))
  (bind _inventory (`self.Inventory`))
  (bind _asbp_base_person (cast `/Game/Blueprints/Characters/Person/BP_BasePerson` Iterator))
  (set `self.IteratorPerson` _asbp_base_person)
  (for (_array_element _array_index) (`/Game/Blueprints/Components/Inventory.Items` _inventory)
    (if (`|EnumInequality` (`.Type_12_E4B9AF6E4BFB737C2F9D1DA63FAC2614` (break `/Game/Blueprints/Structure/F_WasteDetail` (`.Item_7_4E992E384499524884C00BA60CBAADB4` (break `/Game/Blueprints/Structure/F_InventoryWasteSlot` _array_element)))) "NewEnumerator8")
      (bind _wasadded (`/Game/Blueprints/Components/Inventory.TransferItem` (`/Game/Blueprints/Characters/Person/BP_BasePerson.Inventory` (`self.IteratorPerson`)) _array_element))
      (if _wasadded
        (`KismetArrayLibrary.Array_Remove` (`/Game/Blueprints/Components/Inventory.Items` _inventory) _array_index)
        (`/Game/Blueprints/Characters/Person/BP_BasePerson.UpdateInventoryWidget` (`self.IteratorPerson`))
        (`self.UpdateWidget`))))
  (return true))

(fn `UserConstructionScript`)