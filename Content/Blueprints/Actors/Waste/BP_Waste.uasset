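; BP_Waste is a waste item actor that randomly picks its details from DT_WasteCollection on BeginPlay.
; SetWasteDetails weighs a Conscience value, fixed at BeginPlay, against a random roll to choose recyclable or non-recyclable waste.
; It redraws random rows until one matches that recyclability and the first Producer enum value, then stores it in Details.
; Hovering over its Sphere switches the player's cursor to a hand.
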(event `self.ReceiveBeginPlay`
  (`self.SetWasteDetails` 70.0))

(event `self.Sphere.OnBeginCursorOver`
  (params (TouchedComponent :type "PrimitiveComponent Object Reference"))
  ;[1 1 1] Set Default Cursor
  (set `PlayerController.CurrentMouseCursor` "Hand" (`GameplayStatics.GetPlayerController` 0)))

(event `self.Sphere.OnEndCursorOver`
  (params (TouchedComponent :type "PrimitiveComponent Object Reference"))
  ;[1 1 1] Set Default Cursor
  (set `PlayerController.CurrentMouseCursor` "Default" (`GameplayStatics.GetPlayerController` 0)))

(fn `SetWasteDetails`
  (params (Conscience :type "Float (double-precision)"))
  (if (>= Conscience (`KismetMathLibrary.RandomFloatInRange` 0.0 130.0))
    (bind _outrownames (`DataTableFunctionLibrary.GetDataTableRowNames` "/Game/Blueprints/DataTable/DT_WasteCollection.DT_WasteCollection" :!label _label))
    (bind _returnvalue (`|GetDataTableRow` "/Game/Blueprints/DataTable/DT_WasteCollection.DT_WasteCollection" (`|GetArrayItem` _outrownames (`KismetMathLibrary.RandomIntegerInRange` 0 (- (`KismetArrayLibrary.Array_Length` _outrownames) 1))))
      (:`then`
        (bind (_name _description _weight _producer _isrecyclable) (break `/Game/Blueprints/Structure/F_WasteDetail` _returnvalue))
        (if (and (`|EnumEquality` _producer "NewEnumerator0") _isrecyclable)
          (set `self.Details` _returnvalue)
          (else
            (goto _label)))))
    (else
      (bind _outrownames_2 (`DataTableFunctionLibrary.GetDataTableRowNames` "/Game/Blueprints/DataTable/DT_WasteCollection.DT_WasteCollection" :!label _label_2))
      (bind _returnvalue_2 (`|GetDataTableRow` "/Game/Blueprints/DataTable/DT_WasteCollection.DT_WasteCollection" (`|GetArrayItem` _outrownames_2 (`KismetMathLibrary.RandomIntegerInRange` 0 (- (`KismetArrayLibrary.Array_Length` _outrownames_2) 1))))
        (:`then`
          (bind (_name_2 _description_2 _weight_2 _producer_2 _isrecyclable_2) (break `/Game/Blueprints/Structure/F_WasteDetail` _returnvalue_2))
          (if (and (`|EnumEquality` _producer_2 "NewEnumerator0") (not _isrecyclable_2))
            (set `self.Details` _returnvalue_2)
            (else
              (goto _label_2))))))))

(fn `UserConstructionScript`)