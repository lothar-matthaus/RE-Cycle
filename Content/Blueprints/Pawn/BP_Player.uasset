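; Player pawn acting as a top-level camera and input hub, with screen-edge panning, hold-to-rotate look and clamped boom zoom.
; Interact traces under the cursor and sends an interact message to the hit actor.
; BeginPlay adds starting money to the GameState and creates the main HUD, which G swaps for a pause menu.
; Number keys set global game speed, offset by inverse CustomTimeDilation to keep the pawn's own speed roughly constant.
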(event `Key|One`
  (params (Key :type "Key Structure"))
  ;[1 1 1] Set Game Speed
  (:`Pressed`
    (set `self.TimeDilation` 1.0)
    (set `self.CustomTimeDilation` 1.0)
    (`GameplayStatics.SetGlobalTimeDilation` (`self.TimeDilation`) :!label _label)))

(event `Key|Two`
  (params (Key :type "Key Structure"))
  ;[1 1 1] Set Game Speed
  (:`Pressed`
    (set `self.TimeDilation` 3.0)
    (set `self.CustomTimeDilation` 0.35)
    (goto _label)))

(event `Key|Three`
  (params (Key :type "Key Structure"))
  ;[1 1 1] Set Game Speed
  (:`Pressed`
    (set `self.TimeDilation` 5.0)
    (set `self.CustomTimeDilation` 0.2)
    (goto _label)))

(event `self.ReceiveBeginPlay`
  ;[1 1 1] Begin Play
  (set `PlayerCameraManager.ViewPitchMax` 50.0 (`GameplayStatics.GetPlayerCameraManager` 0))
  (bind _returnvalue (`GameplayStatics.GetActorOfClass` "/Game/Blueprints/Components/Level/BP_LevelDayTime.BP_LevelDayTime_C"))
  (set `self.DayTime` _returnvalue)
  (set `self.GameState` (cast `/Game/Blueprints/Game/BP_GameState` (`GameplayStatics.GetGameState`) :!pure true))
  (`self.IncrementPlayerMoney` 1200.0)
  (`self.CreateMainWidget`))

(event `self.ReceiveTick`
  (params (DeltaSeconds :type "Float (single-precision)"))
  ;[1 1 1] Event Tick
  (`|ExecutionSequence`
    (:`then_0`
      (bind (_forward_value _right_value) (`self.Calculate Mouse Position`))
      (set `self.ForwardValue` _forward_value)
      (set `self.RightValue` _right_value)
      (if (`self.CanMovePawn`)
        (`|ExecutionSequence`
          (:`then_0`
            (`self.Move Forward` (`self.ForwardValue`)))
          (:`then_1`
            (`self.Move Right` (`self.RightValue`))))))))

(event `Move Forward`
  (params (ForwardValue :type "Float (double-precision)"))
  ;[1 1 1] Camera Movement
  (`self.AddMovementInput` (`KismetMathLibrary.GetForwardVector` (`KismetMathLibrary.MakeRotator` (.roll (`self.GetControlRotation`)) 0.0 (.yaw (`self.GetControlRotation`)))) ForwardValue))

(event `InputAction|ManipulateCamera`
  (params (Key :type "Key Structure"))
  ;[1 1 1] Camera Controll
  (:`Pressed`
    (set `self.ManipulateCamera` true))
  (:`Released`
    (set `self.ManipulateCamera` false)))

(event `InputAxis|LookAround`
  (params (AxisValue :type "Float (single-precision)"))
  ;[1 1 1] Camera Controll
  (if (`self.ManipulateCamera`)
    (`self.AddControllerYawInput` AxisValue)))

(event `Move Right`
  (params (RightValue :type "Float (double-precision)"))
  ;[1 1 1] Camera Movement
  (`self.AddMovementInput` (`KismetMathLibrary.GetRightVector` (`KismetMathLibrary.MakeRotator` (.roll (`self.GetControlRotation`)) 0.0 (.yaw (`self.GetControlRotation`)))) RightValue))

(event `InputAxis|LookUp`
  (params (AxisValue :type "Float (single-precision)"))
  ;[1 1 1] Camera Controll
  (if (`self.ManipulateCamera`)
    (`self.AddControllerPitchInput` AxisValue)))

(event `InputAction|ZoomIn`
  (params (Key :type "Key Structure"))
  (bind _cameraboom (`self.CameraBoom`))
  ;[1 1 1] ZoomIn Settings
  (:`Pressed`
    (set `SpringArmComponent.TargetArmLength` (`KismetMathLibrary.FClamp` (- (`SpringArmComponent.TargetArmLength` _cameraboom) (`self.ZoomRate`)) (`self.MaxZoomInRate`) (`self.MaxZoomOutRate`)) _cameraboom)))

(event `InputAction|ZoomOut`
  (params (Key :type "Key Structure"))
  (bind _cameraboom (`self.CameraBoom`))
  ;[1 1 1] ZoomOut Settings
  (:`Pressed`
    (set `SpringArmComponent.TargetArmLength` (`KismetMathLibrary.FClamp` (+ (`SpringArmComponent.TargetArmLength` _cameraboom) (`self.ZoomRate`)) (`self.MaxZoomInRate`) (`self.MaxZoomOutRate`)) _cameraboom)))

(event `ChangePlayerCursor`
  (bind (_hitresult _returnvalue) (`PlayerController.GetHitResultUnderCursorForObjects` (`GameplayStatics.GetPlayerController` 0) (`|MakeArray` "ObjectTypeQuery2" "ObjectTypeQuery3" :!type "EObjectTypeQuery Enum") true))
  ;[1 1 1] Interact Settings
  (if _returnvalue :!label _label_2
    (message `/Game/Blueprints/Interfaces/BI_Interactable.Interact` (`.HitActor` (`GameplayStatics.BreakHitResult` _hitresult)) self)))

(event `InputAction|Interact`
  (params (Key :type "Key Structure"))
  ;[1 1 1] Interact Settings
  (:`Pressed`
    (goto _label_2)))

(event `CreateMainWidget`
  ;[1 1 1] Creating Global Widget
  (bind _returnvalue (`|CreateWidget` "/Game/Blueprints/UI/WPB_Main.WPB_Main_C" (`GameplayStatics.GetPlayerController` 0)))
  (bind _output_get (set `self.MainWidget` _returnvalue))
  (`/Game/Blueprints/UI/WPB_Main.SetData` _output_get (`self.GameState`) self)
  (`UserWidget.AddToViewport` _output_get 0)
  (set `self.WBPPauseMenu` null))

(event `Key|G`
  (params (Key :type "Key Structure"))
  ;[1 1 1] Pause Game
  (:`Pressed`
    (`/Engine/EditorBlueprintResources/StandardMacros.IsValid` (`self.WBPPauseMenu`)
      (:`Is Not Valid`
        (`Widget.RemoveFromParent` (`self.MainWidget`))
        (bind _returnvalue (`|CreateWidget` "/Game/Blueprints/UI/WBP_PauseMenu.WBP_PauseMenu_C" (`GameplayStatics.GetPlayerController` 0)))
        (bind _output_get (set `self.WBPPauseMenu` _returnvalue))
        (`UserWidget.AddToViewport` _output_get 0)
        (set `/Game/Blueprints/UI/WBP_PauseMenu.PawnReference` self (`self.WBPPauseMenu`))))))

(fn `Calculate Mouse Position`
  (returns (`Forward Value` :type "Float (double-precision)") (`Right Value` :type "Float (double-precision)"))
  (locals (XPosition :type "Float (double-precision)") (YPosition :type "Float (double-precision)"))
  (bind (_x _y) (`KismetMathLibrary.BreakVector2D` (`WidgetLayoutLibrary.GetViewportSize`)))
  (bind (_locationx _locationy) (`PlayerController.GetMousePosition` (`GameplayStatics.GetPlayerController` 0)))
  (bind _returnvalue (/ _locationy _y))
  (bind _returnvalue_2 (/ _locationx _x))
  (`|ExecutionSequence`
    (:`then_0`
      (if (<= _returnvalue_2 0.0)
        (set `local.XPosition` -1.0)
        (elif (>= _returnvalue_2 0.99)
          (set `local.XPosition` 1.0)
          (else
            (set `local.XPosition` 0.0)))))
    (:`then_1`
      (if (<= _returnvalue 0.0)
        (set `local.YPosition` 1.0)
        (elif (>= _returnvalue 0.99)
          (set `local.YPosition` -1.0)
          (else
            (set `local.YPosition` 0.0)))))
    (:`then_2`
      (return (`local.YPosition`) (`local.XPosition`)))))

(fn `IncrementPlayerMoney`
  (params (Budget :type "Float (double-precision)"))
  (bind _output_get (set `self.Budget` (+ Budget (`self.Budget`))))
  (setmembers `/Game/Blueprints/Structure/F_OverallInfo` :`StructRef` (`/Game/Blueprints/Game/BP_GameState.OverallInfo` (`self.GameState`)) :`TotalRaisedBudget` _output_get))

(fn `UserConstructionScript`)