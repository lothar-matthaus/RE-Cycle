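; Game state for a neighborhood waste-management game that runs random objectives and accumulates overall stats.
; BeginPlay picks three distinct DT_Objectives rows with random future days, then a one-second timer checks deadlines and progress.
; Description text selects each goal check against OverallInfo totals or world actors.
; Settled objectives show WBP_Objective, with successes granting rewards to residents, budget or streets by reward text.
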(event `self.ReceiveBeginPlay`
  (bind _returnvalue (`GameplayStatics.GetActorOfClass` "/Game/Blueprints/Components/Level/BP_LevelDayTime.BP_LevelDayTime_C"))
  (set `self.DayTimeComponent` _returnvalue)
  (`self.GenerateObjectives`)
  (`KismetSystemLibrary.K2_SetTimer` null "UpdateObjectiveProgressEvent" 1.0 true))

(event `UpdateObjectiveProgressEvent`
  (`self.UpdateObjectiveProgress`))

(fn `CreateWidgetMessageCompleted`
  (params (Objective :type "/Game/Blueprints/Structure/F_Objective Structure"))
  (locals (WidgetCompleteWindow :type "/Game/Blueprints/UI/Objectives/WBP_Objective Object Reference"))
  (bind _returnvalue (`|CreateWidget` "/Game/Blueprints/UI/Objectives/WBP_Objective.WBP_Objective_C" (`GameplayStatics.GetPlayerController` 0)))
  (bind _output_get (set `local.WidgetCompleteWindow` _returnvalue))
  (`/Game/Blueprints/UI/Objectives/WBP_Objective.SetObjective` _output_get Objective false)
  (`UserWidget.AddToViewport` _output_get 0))

(fn `GenerateObjectives`
  (locals (Day :type Integer) (RewardValue :type Integer) (GoalValue :type Integer) (Description :type String) (Type :type Byte) (RewardDescription :type String) (Objective :type "/Game/Blueprints/Structure/F_Objective Structure") (CurrentDay :type Integer :default 0) (ObjectiveCanBeAdded :type Boolean))
  (bind _currentday (`local.CurrentDay`))
  (bind _objectives (`self.Objectives`))
  (for _ (range 3)
    (bind _outrownames (`DataTableFunctionLibrary.GetDataTableRowNames` "/Game/Blueprints/DataTable/DT_Objectives.DT_Objectives" :!label _label))
    (bind _returnvalue (`|GetDataTableRow` "/Game/Blueprints/DataTable/DT_Objectives.DT_Objectives" (`|GetArrayItem` _outrownames (`KismetMathLibrary.RandomIntegerInRange` 0 (- (`KismetArrayLibrary.Array_Length` _outrownames) 1))))
      (:`then`
        (set `local.Objective` _returnvalue)
        (if (not (`KismetArrayLibrary.Array_IsEmpty` _objectives))
          (for _array_element _objectives
            (if (`|EnumEquality` (`.Description_34_9691BA284AF455659920CE8E1F480366` (break `/Game/Blueprints/Structure/F_Objective` _array_element)) (`.Description_34_9691BA284AF455659920CE8E1F480366` (break `/Game/Blueprints/Structure/F_Objective` (`local.Objective`))))
              (set `local.ObjectiveCanBeAdded` false)
              (break)
              (else
                (set `local.ObjectiveCanBeAdded` true))))
          (if (`local.ObjectiveCanBeAdded`)
            _
            (else
              (goto _label))))
        (bind _day (`/Game/Blueprints/Components/Level/BP_LevelDayTime.GetCurrentDay` (`self.DayTimeComponent`)))
        (set `local.CurrentDay` _day)
        (bind _structout (setmembers `/Game/Blueprints/Structure/F_Objective` :`StructRef` (`local.Objective`) :`Day` (`KismetMathLibrary.RandomIntegerInRange` (+ _currentday 10) (+ _currentday 50))))
        (`KismetArrayLibrary.Array_Add` (`self.Objectives`) _structout)))))

(fn `GetObjectives`
  (returns (Objectives :type "Array of /Game/Blueprints/Structure/F_Objective Structure"))
  (return (`self.Objectives`)))

(fn `SettleObjective`
  (params (ObjectiveToSettle :type "/Game/Blueprints/Structure/F_Objective Structure") (ArrayIndex :type Integer))
  (locals (Objective :type "/Game/Blueprints/Structure/F_Objective Structure") (Index :type Integer))
  (bind _objective (`local.Objective`))
  (bind _objective_2 (`local.Objective`))
  (bind _output_get (set `local.Objective` ObjectiveToSettle))
  (set `local.Index` ArrayIndex)
  (bind ((`GoalValue_51_0E20DEB4426C52BCBE665ABB74ED0B95` _goalvalue) (`CurrentGoalValue_52_0B043DC943190198253EE5A0B663B650` _currentgoalvalue) (`Success_43_31B50596445D49F7A13B65B48663DD42` _success) (`Completed_44_66CD1431471BAFF4F1AA9F83FCB7DC51` _completed) (`RewardValue_50_BAF293AD46816B8B8A84ED8F8763FA11` _rewardvalue) (`RewardDescription_36_F5523ADD472C78516820458DBFBF403D` _rewarddescription)) (break `/Game/Blueprints/Structure/F_Objective` _output_get))
  (if (and _success (not _completed))
    (bind _foundwidgets (`WidgetBlueprintLibrary.GetAllWidgetsOfClass` "/Game/Blueprints/UI/Objectives/WBP_Objective.WBP_Objective_C"))
    (bind _returnvalue (== (`KismetArrayLibrary.Array_Length` _foundwidgets) 0))
    (if _returnvalue
      (`self.CreateWidgetMessageCompleted` (`local.Objective`))
      (switch `/Game/Blueprints/Enum/E_Reward` _rewarddescription
        (:`NewEnumerator0`
          (bind _outactors (`GameplayStatics.GetAllActorsOfClass` "/Game/Blueprints/Characters/Resident/BP_Resident.BP_Resident_C"))
          (for _array_element _outactors
            (`/Game/Blueprints/Characters/Person/BP_BasePerson.IncrementConscience` _array_element (`.RewardValue_50_BAF293AD46816B8B8A84ED8F8763FA11` (break `/Game/Blueprints/Structure/F_Objective` (`local.Objective`)))))
          (`self.UpdateObjectiveStatus` (`local.Objective`) (`local.Index`)))
        (:`NewEnumerator1`
          (bind _asbp_player (cast `/Game/Blueprints/Pawn/BP_Player` (`GameplayStatics.GetPlayerPawn` 0)))
          (set `/Game/Blueprints/Pawn/BP_Player.Budget` (+ (`/Game/Blueprints/Pawn/BP_Player.Budget` _asbp_player) (`.RewardValue_50_BAF293AD46816B8B8A84ED8F8763FA11` (break `/Game/Blueprints/Structure/F_Objective` (`local.Objective`)))) _asbp_player)
          (`self.UpdateObjectiveStatus` (`local.Objective`) (`local.Index`)))
        (:`NewEnumerator2`
          (bind _outactors_2 (`GameplayStatics.GetAllActorsOfClass` "/Game/Blueprints/Actors/Waste/BP_Waste.BP_Waste_C"))
          (for _array_element_2 _outactors_2
            (`self.K2_DestroyActor` _array_element_2))
          (`self.UpdateObjectiveStatus` (`local.Objective`) (`local.Index`)))
        (:`NewEnumerator3`
          (bind _outactors_3 (`GameplayStatics.GetAllActorsOfClass` "/Game/Blueprints/Characters/Resident/BP_Resident.BP_Resident_C"))
          (for _array_element_3 _outactors_3
            (`/Game/Blueprints/Characters/Person/BP_BasePerson.IncrementMood` _array_element_3 (`.RewardValue_50_BAF293AD46816B8B8A84ED8F8763FA11` (break `/Game/Blueprints/Structure/F_Objective` _objective_2))))
          (`self.UpdateObjectiveStatus` _objective_2 (`local.Index`)))
        (:`NewEnumerator4`
          (bind _outactors_4 (`GameplayStatics.GetAllActorsOfClass` "/Game/Blueprints/Characters/Resident/BP_Resident.BP_Resident_C"))
          (for _array_element_4 _outactors_4
            (set `/Game/Blueprints/Characters/Person/BP_BasePerson.ConscienceIncrementRate` (+ (/ (`.RewardValue_50_BAF293AD46816B8B8A84ED8F8763FA11` (break `/Game/Blueprints/Structure/F_Objective` _objective)) 100.0) (`/Game/Blueprints/Characters/Person/BP_BasePerson.ConscienceIncrementRate` _array_element_4)) _array_element_4))
          (`self.UpdateObjectiveStatus` _objective (`local.Index`)))))
    (elif _returnvalue
      (`self.CreateWidgetMessageCompleted` (`local.Objective`)))))

(fn `UpdateObjectiveProgress`
  (locals (Index :type Integer) (Objective :type "/Game/Blueprints/Structure/F_Objective Structure"))
  (if (not (== (`KismetArrayLibrary.Array_Length` (`self.Objectives`)) 0))
    (for (_array_element _array_index) (`self.Objectives`)
      (set `local.Index` _array_index)
      (set `local.Objective` _array_element)
      (bind ((`Description_34_9691BA284AF455659920CE8E1F480366` _description) (`GoalValue_51_0E20DEB4426C52BCBE665ABB74ED0B95` _goalvalue) (`CurrentGoalValue_52_0B043DC943190198253EE5A0B663B650` _currentgoalvalue) (`Completed_44_66CD1431471BAFF4F1AA9F83FCB7DC51` _completed) (`Day_22_ECD822CC4B895CEFA4CA2ABFCBFF3A33` _day) (`HasDeadLine_49_4841EA3542FFB402AFB02A94C9E1DAED` _hasdeadline)) (break `/Game/Blueprints/Structure/F_Objective` _array_element))
      (if (not _completed)
        (if (and (< _day (`/Game/Blueprints/Components/Level/BP_LevelDayTime.Day` (`self.DayTimeComponent`))) _hasdeadline)
          (setmembers `/Game/Blueprints/Structure/F_Objective` :`StructRef` (`local.Objective`) :`Success` false :`Completed` true)
          (`KismetArrayLibrary.Array_Set` (`self.Objectives`) (`local.Index`) (`local.Objective`))
          (`self.SettleObjective` (`local.Objective`) (`local.Index`))
          (break)
          (else
            (`|ExecutionSequence`
              (:`then_0`
                (switch `/Game/Blueprints/Enum/E_Objective` _description
                  (:`NewEnumerator3`
                    (bind _outactors (`GameplayStatics.GetAllActorsOfClass` "/Game/Blueprints/Actors/House/BP_BaseHouse.BP_BaseHouse_C"))
                    (for _array_element_2 _outactors
                      (bind _conscience (`/Game/Blueprints/Actors/House/BP_BaseHouse.GetAverageConscience` _array_element_2))
                      (if (> _conscience (`.CurrentGoalValue_52_0B043DC943190198253EE5A0B663B650` (break `/Game/Blueprints/Structure/F_Objective` (`local.Objective`))))
                        (`self.TryToCompleteObjective` (`local.Objective`) (`local.Index`) (`self.Objectives`) _conscience
                          (:`out`
                            (break))))))
                  (:`NewEnumerator4`
                    (`self.TryToCompleteObjective` (`local.Objective`) (`local.Index`) (`self.Objectives`) (`KismetMathLibrary.Conv_IntToDouble` (`.TotalRunnedCampaigns_83_8A690A944D725E50CB590EB13132E7D3` (break `/Game/Blueprints/Structure/F_OverallInfo` (`self.OverallInfo`))))))
                  (:`NewEnumerator5`
                    (`self.TryToCompleteObjective` (`local.Objective`) (`local.Index`) (`self.Objectives`) (`.TotalRecyclableWasteWeight_56_BE899F404B2463B50D1250AE1D050569` (break `/Game/Blueprints/Structure/F_OverallInfo` (`self.OverallInfo`)))))
                  (:`NewEnumerator6`
                    (`self.TryToCompleteObjective` (`local.Objective`) (`local.Index`) (`self.Objectives`) (`KismetMathLibrary.Conv_IntToDouble` (`.TotalHiredSweepers_79_27A9A5094771E38D11C419BCD677A991` (break `/Game/Blueprints/Structure/F_OverallInfo` (`self.OverallInfo`))))))
                  (:`NewEnumerator7`
                    (`self.TryToCompleteObjective` (`local.Objective`) (`local.Index`) (`self.Objectives`) (`KismetMathLibrary.Conv_IntToDouble` (`.TotalHiredCollectors_82_95B1C9A2489EF22774913D95EB478C10` (break `/Game/Blueprints/Structure/F_OverallInfo` (`self.OverallInfo`))))))
                  (:`NewEnumerator8`
                    (bind _outactors_2 (`GameplayStatics.GetAllActorsOfClass` "/Game/Blueprints/Actors/TrashBin/BP_Composter.BP_Composter_C"))
                    (`self.TryToCompleteObjective` (`local.Objective`) (`local.Index`) (`self.Objectives`) (`KismetMathLibrary.Conv_IntToDouble` (`KismetArrayLibrary.Array_Length` _outactors_2))))
                  (:`NewEnumerator9`
                    (`self.TryToCompleteObjective` (`local.Objective`) (`local.Index`) (`self.Objectives`) (`.TotalRaisedBudget_90_387ACB05497837851E5FEFB6EDA85F01` (break `/Game/Blueprints/Structure/F_OverallInfo` (`self.OverallInfo`)))))
                  (:`NewEnumerator10`
                    (`self.TryToCompleteObjective` (`local.Objective`) (`local.Index`) (`self.Objectives`) (`KismetMathLibrary.Conv_IntToDouble` (`.TotalActiveSweepers_80_7DF9B0B245326A1C53D940870D907458` (break `/Game/Blueprints/Structure/F_OverallInfo` (`self.OverallInfo`))))))))
              (:`then_1`
                (if (`.Success_43_31B50596445D49F7A13B65B48663DD42` (break `/Game/Blueprints/Structure/F_Objective` (`local.Objective`)))
                  (`self.SettleObjective` (`local.Objective`) (`local.Index`))
                  (break))))))))))

(fn `UpdateObjectiveStatus`
  (params (Objective :type "/Game/Blueprints/Structure/F_Objective Structure (by ref)") (Index :type Integer))
  (bind _structout (setmembers `/Game/Blueprints/Structure/F_Objective` :`StructRef` Objective :`Completed` true))
  (`KismetArrayLibrary.Array_Set` (`self.Objectives`) (`local.Index`) _structout))

(fn `UpdateOverallInfo`
  (params (Stats :type "/Game/Blueprints/Structure/F_OverallInfo Structure"))
  (bind (_totalorganicwasteweight _totalrecyclablewasteweight _totalwasteweigh _totalrecyclableprice _totalweightgenerated _totalbudget _totalraisedbudget _totalhiredsweepers _totalactivesweepers _totalhiredcollectors _totalactivecollectors _totalrunnedcampaigns _totalactivecampaigns) (break `/Game/Blueprints/Structure/F_OverallInfo` Stats))
  (bind (_totalorganicwasteweight_2 _totalrecyclablewasteweight_2 _totalwasteweigh_2 _totalrecyclableprice_2 _totalweightgenerated_2 _totalbudget_2 _totalraisedbudget_2 _totalhiredsweepers_2 _totalactivesweepers_2 _totalhiredcollectors_2 _totalactivecollectors_2 _totalrunnedcampaigns_2 _totalactivecampaigns_2) (break `/Game/Blueprints/Structure/F_OverallInfo` (`self.OverallInfo`)))
  (setmembers `/Game/Blueprints/Structure/F_OverallInfo` :`StructRef` (`self.OverallInfo`) :`TotalOrganicWasteWeight` (+ _totalorganicwasteweight _totalorganicwasteweight_2) :`TotalRecyclableWasteWeight` (+ _totalrecyclablewasteweight _totalrecyclablewasteweight_2) :`TotalWasteWeigh` (+ _totalwasteweigh _totalwasteweigh_2) :`TotalRecyclablePrice` (+ _totalrecyclableprice _totalrecyclableprice_2) :`TotalWeightGenerated` (+ _totalweightgenerated _totalweightgenerated_2) :`TotalBudget` (+ _totalbudget _totalbudget_2) :`TotalRaisedBudget` (+ _totalraisedbudget _totalraisedbudget_2) :`TotalHiredSweepers` (+ _totalhiredsweepers _totalhiredsweepers_2) :`TotalActiveSweepers` (+ _totalactivesweepers _totalactivesweepers_2) :`TotalHiredCollectors` (+ _totalhiredcollectors _totalhiredcollectors_2) :`TotalActiveCollectors` (+ _totalactivecollectors _totalactivecollectors_2) :`TotalRunnedCampaigns` (+ _totalrunnedcampaigns _totalrunnedcampaigns_2) :`TotalActiveCampaigns` (+ _totalactivecampaigns _totalactivecampaigns_2)))

(fn `UserConstructionScript`)