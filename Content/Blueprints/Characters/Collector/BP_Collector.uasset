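; Collector character, a hired service NPC with a timed lifespan, built on a parent person class.
; On BeginPlay it reads its duration from DT_Services, runs BT_Collector, sets person details and spawn point, and registers as hired and active with BP_GameState.
; A looping one-second timer counts Lifespan down while DecreaseLifespan is set, updating the overhead PersonIcon widget.
; Destruction sends a zero-budget info update to the game state.
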(event `self.ReceiveBeginPlay`
  (`parent.ReceiveBeginPlay`)
  (`self.SetLifeSpan` 0.0)
  (bind _returnvalue (`|GetDataTableRow` "/Game/Blueprints/DataTable/DT_Services.DT_Services" "Collector")
    (:`then`
      (bind ((`Duration_11_F3B0E8F94D2078569F9CE5B3D227ED6E` _duration)) (break `/Game/Blueprints/Structure/F_Service` _returnvalue))
      (set `self.MaxLifespan` _duration)
      (set `self.Lifespan` _duration)
      (`AIController.RunBehaviorTree` (`AIBlueprintHelperLibrary.GetAIController` self) "/Game/Blueprints/AI/Collector/BT_Collector.BT_Collector")
      (`self.SetPersonDetails`)
      (`self.SetSpawnPoint`)
      (bind _aswbp_person_icon (cast `/Game/Blueprints/UI/Person/WBP_PersonIcon` (`WidgetComponent.GetWidget` (`self.TimeWidget`))))
      (bind _output_get (set `self.WBP_TimeWidge` _aswbp_person_icon))
      (`/Game/Blueprints/UI/Person/WBP_PersonIcon.Set Time` _output_get (`self.Lifespan`) (`self.MaxLifespan`))
      (`KismetSystemLibrary.K2_SetTimer` null "UpdateLifespan" 1.0 true)
      (bind _asbp_game_state (cast `/Game/Blueprints/Game/BP_GameState` (`GameplayStatics.GetGameState`)))
      (set `self.GameState` _asbp_game_state)
      (`/Game/Blueprints/Game/BP_GameState.UpdateOverallInfo` (`self.GameState`) (make `/Game/Blueprints/Structure/F_OverallInfo` :`TotalHiredCollectors` 1 :`TotalActiveCollectors` 1)))))

(event `UpdateLifespan`
  (bind _lifespan (`self.Lifespan`))
  (if (`self.bDecreaseLifespan`)
    (bind _output_get (set `self.Lifespan` (`KismetMathLibrary.FClamp` (- _lifespan 1.0) 0.0 _lifespan)))
    (`/Game/Blueprints/UI/Person/WBP_PersonIcon.Set Time` (`self.WBP_TimeWidge`) _output_get (`self.MaxLifespan`))))

(event `self.ReceiveDestroyed`
  (`/Game/Blueprints/Game/BP_GameState.UpdateOverallInfo` (`self.GameState`) (make `/Game/Blueprints/Structure/F_OverallInfo` :`TotalHiredCollectors` -1 :`TotalActiveCollectors` -1)))

(fn `SetPersonDetails`
  (setmembers `/Game/Blueprints/Structure/F_PersonDetail` :`StructRef` (`self.Details`) :`Conscience` 100.0 :`Mood` 100.0)
  (`parent.SetPersonDetails`))

(fn `UserConstructionScript`
  (`parent.UserConstructionScript`))