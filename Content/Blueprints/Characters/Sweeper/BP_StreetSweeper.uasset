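; BP_StreetSweeper is a street sweeper character driven by the BT_StreetSweeper behavior tree.
; On BeginPlay it starts the tree on its AI controller, sets its person details and swaps in a shopkeeper skeletal mesh.
; Its SetPersonDetails override randomizes Conscience in the person details struct before calling the parent version.
; GenerateWaste is left empty, so that function produces no waste.
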(event `self.ReceiveBeginPlay`
  (`AIController.RunBehaviorTree` (`AIBlueprintHelperLibrary.GetAIController` self) "/Game/Blueprints/AI/BT_StreetSweeper.BT_StreetSweeper")
  (`self.SetPersonDetails`)
  (`SkinnedMeshComponent.SetSkinnedAssetAndUpdate` (`self.Mesh`) "/Game/Import/PolygonTown/Meshes/Characters/SK_Character_ShopKeeper_01.SK_Character_ShopKeeper_01" true))

(fn `Generate Waste`)

(fn `SetPersonDetails`
  (setmembers `/Game/Blueprints/Structure/F_PersonDetail` :`StructRef` (`self.Details`) :`Conscience` (`KismetMathLibrary.RandomFloatInRange` 10.0 30.0))
  (`parent.SetPersonDetails`))

(fn `UserConstructionScript`
  (`parent.UserConstructionScript`))