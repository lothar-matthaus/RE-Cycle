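; Base person character for a waste-management game, with cursor hover feedback and an info widget shown on interaction.
; SetPersonDetails randomizes age, gender and data-table names, then picks a matching skeletal mesh.
; GenerateWaste spawns BP_Waste from the person's Conscience, updates person, residence and GameState totals, and stores it in the residence or personal inventory.
; Recyclable waste raises Conscience, which also feeds awareness points to GameState.
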(event `self.ReceiveBeginPlay`
  ;[1 1 1] Initialize Person
  (bind _asbp_game_state (cast `/Game/Blueprints/Game/BP_GameState` (`GameplayStatics.GetGameState`))
    (:`then`
      (set `self.GameState` _asbp_game_state))
    (:`CastFailed`
      _))
  (`self.SetSpawnPoint`))

(event `/Game/Blueprints/Interfaces/BI_Interactable.Interact`
  (params (Interactor :type "Actor Object Reference (by ref)"))
  (bind _personinfo (`self.PersonInfo`))
  ;[1 1 1] Show Person Info
  (if (not (`SceneComponent.IsVisible` _personinfo))
    (bind _returnvalue (`|CreateWidget` "/Game/Blueprints/UI/Person/WBP_PersonInfo.WBP_PersonInfo_C"))
    (`WidgetComponent.SetWidget` _personinfo _returnvalue)
    (`/Game/Blueprints/UI/Person/WBP_PersonInfo.SetPersonReference` _returnvalue self)
    (`SceneComponent.SetVisibility` _personinfo true true)))

(event `self.CapsuleComponent.OnBeginCursorOver`
  (params (TouchedComponent :type "PrimitiveComponent Object Reference"))
  ;[1 1 1] Change Default Cursor
  (set `PlayerController.CurrentMouseCursor` "Hand" (`GameplayStatics.GetPlayerController` 0)))

(event `self.CapsuleComponent.OnEndCursorOver`
  (params (TouchedComponent :type "PrimitiveComponent Object Reference"))
  ;[1 1 1] Change Default Cursor
  (set `PlayerController.CurrentMouseCursor` "Default" (`GameplayStatics.GetPlayerController` 0)))

(fn `Generate Waste`
  (locals (LocalWaste :type "/Game/Blueprints/Actors/Waste/BP_Waste Object Reference"))
  (bind _localwaste (`local.LocalWaste`))
  (bind _gamestate (`self.GameState`))
  (bind ((`Residence_46_D0366B25453D32004AFFDB8FED01C469` _residence)) (break `/Game/Blueprints/Structure/F_PersonDetail` (`self.Details`)))
  (bind ((`Conscience_35_519E32E14799A62A65B328B0DD622DAE` _conscience) (`Residence_46_D0366B25453D32004AFFDB8FED01C469` _residence_2)) (break `/Game/Blueprints/Structure/F_PersonDetail` (`self.Details`)))
  (bind ((`Residence_46_D0366B25453D32004AFFDB8FED01C469` _residence_3)) (break `/Game/Blueprints/Structure/F_PersonDetail` (`self.Details`)))
  (bind ((`Task_43_E546C9C543F5E34D866A2DAFCA92E390` _task)) (break `/Game/Blueprints/Structure/F_PersonDetail` (`self.Details`)))
  (bind _returnvalue (* (`self.ConscienceIncrementRate`) 5.0))
  (if (not (or (`|EnumEquality` _task "NewEnumerator3") (`|EnumEquality` _task "NewEnumerator12")))
    (switch `/Game/Blueprints/Enum/E_PersonType` (`.Type_42_E4120F5346141B9F587952AB352393B3` (break `/Game/Blueprints/Structure/F_PersonDetail` (`self.Details`)))
      (:`NewEnumerator0`
        _)
      (:`NewEnumerator1`
        _))
    (bind _returnvalue_2 (`|SpawnActorFromClass` "/Game/Blueprints/Actors/Waste/BP_Waste.BP_Waste_C" (`KismetMathLibrary.Conv_VectorToTransform` (`SceneComponent.K2_GetComponentLocation` (`self.WasteSpawn`))) "AdjustIfPossibleButAlwaysSpawn" "OverrideRootScale" null null))
    (bind _output_get (set `local.LocalWaste` _returnvalue_2))
    (`/Game/Blueprints/Actors/Waste/BP_Waste.SetWasteDetails` _output_get _conscience)
    (bind _statstoexportparam (`self.UpdatePersonStats` _localwaste))
    (`/Engine/EditorBlueprintResources/StandardMacros.IsValid` _gamestate
      (:`Is Valid`
        (`/Game/Blueprints/Game/BP_GameState.UpdateOverallInfo` _gamestate _statstoexportparam))
      (:`Is Not Valid`
        _))
    (`/Engine/EditorBlueprintResources/StandardMacros.IsValid` _residence_2
      (:`Is Valid`
        (`/Game/Blueprints/Actors/House/BP_BaseHouse.UpdateHouseStats` _residence_2 _output_get))
      (:`Is Not Valid`
        _))
    (if (`.IsRecyclable_30_ACD23FA84E311774B1F025BB1F87331C` (break `/Game/Blueprints/Structure/F_WasteDetail` (`/Game/Blueprints/Actors/Waste/BP_Waste.Details` _localwaste)))
      (`self.IncrementConscience` _returnvalue)
      (if (`|EnumEquality` (`.Type_42_E4120F5346141B9F587952AB352393B3` (break `/Game/Blueprints/Structure/F_PersonDetail` (`self.Details`))) "NewEnumerator0")
        (`/Game/Blueprints/Game/BP_GameState.UpdateOverallInfo` (`self.GameState`) (make `/Game/Blueprints/Structure/F_OverallInfo` :`TotalAwarenessPoints` _returnvalue))))
    (if (`self.IsOverlappingActor` _residence_3)
      (`/Game/Blueprints/Components/Inventory.AddToInventory` (`/Game/Blueprints/Actors/House/BP_BaseHouse.Inventory` _residence_3) (`local.LocalWaste`))
      (`self.UpdateInventoryWidget`)
      (message `/Game/Blueprints/Interfaces/BI_Widget.UpdateWidget` _residence)
      (else
        (`/Game/Blueprints/Components/Inventory.AddToInventory` (`self.Inventory`) (`local.LocalWaste`))
        (`self.UpdateInventoryWidget`)
        (message `/Game/Blueprints/Interfaces/BI_Widget.UpdateWidget` _residence)))))

(fn `GetName`
  (returns (Name :type Text))
  (return (`KismetTextLibrary.Conv_StringToText` (`.Name_33_DBD6BC6C477B0B035D13248568F853BC` (break `/Game/Blueprints/Structure/F_PersonDetail` (`self.Details`))))))

(fn `IncrementConscience`
  (params (Amount :type "Float (double-precision)"))
  (bind _details (`self.Details`))
  (setmembers `/Game/Blueprints/Structure/F_PersonDetail` :`StructRef` _details :`Conscience` (`KismetMathLibrary.FClamp` (+ Amount (`.Conscience_35_519E32E14799A62A65B328B0DD622DAE` (break `/Game/Blueprints/Structure/F_PersonDetail` _details))) 0.0 100.0))
  (`/Game/Blueprints/Game/BP_GameState.UpdateOverallInfo` (`self.GameState`) (make `/Game/Blueprints/Structure/F_OverallInfo` :`TotalAwarenessPoints` (`local.Amount`))))

(fn `IncrementMood`
  (params (Amount :type "Float (double-precision)"))
  (bind _details (`self.Details`))
  (setmembers `/Game/Blueprints/Structure/F_PersonDetail` :`StructRef` _details :`Mood` (`KismetMathLibrary.FClamp` (+ Amount (`.Mood_36_7BCD7D5140C9C277061647BB3AC58066` (break `/Game/Blueprints/Structure/F_PersonDetail` _details))) 0.0 100.0)))

(fn `RemoveWidget`
  (bind _personinfo (`self.PersonInfo`))
  (`WidgetComponent.SetWidget` _personinfo null)
  (`SceneComponent.SetVisibility` _personinfo false true))

(fn `SetMesh`
  (bind (_f_charactermesh_m_adultmesh _f_charactermesh_m_teenagermesh _f_charactermesh_f_adultmesh _f_charactermesh_f_teenagermesh) (break `/Game/Blueprints/Structure/F_CharacterMesh` (make `/Game/Blueprints/Structure/F_CharacterMesh`)))
  (bind (_details_name _details_lastname _details_conscience _details_gender _details_age _details_agegroup) (break `/Game/Blueprints/Structure/F_PersonDetail` (`self.Details`)))
  (switch `/Game/Blueprints/Enum/E_Gender` _details_gender
    (:`NewEnumerator2`
      (switch `/Game/Blueprints/Enum/E_AgeGroup` _details_agegroup
        (:`NewEnumerator1`
          (`self.SetCharacterMesh` _f_charactermesh_m_teenagermesh))
        (:`NewEnumerator2`
          (`self.SetCharacterMesh` _f_charactermesh_m_adultmesh))))
    (:`NewEnumerator1`
      (switch `/Game/Blueprints/Enum/E_AgeGroup` _details_agegroup
        (:`NewEnumerator1`
          (`self.SetCharacterMesh` _f_charactermesh_f_teenagermesh))
        (:`NewEnumerator2`
          (`self.SetCharacterMesh` _f_charactermesh_f_adultmesh))))))

(fn `SetPersonDetails`
  (locals (Gender :type "/Game/Blueprints/Enum/E_Gender Enum") (Name :type String) (LastName :type String) (Age :type Integer) (Conscience :type "Float (double-precision)") (AgeGroup :type "/Game/Blueprints/Enum/E_AgeGroup Enum") (Mood :type "Float (double-precision)") (Type :type "/Game/Blueprints/Enum/E_PersonType Enum"))
  (bind _output_get (set `local.Age` (`KismetMathLibrary.RandomIntegerInRange` 14 38)))
  (bind _agegroup (`self.SetPersonAgeGroup` _output_get))
  (set `local.AgeGroup` _agegroup)
  (bind _output_get_2 (set `local.Gender` (cast `/Game/Blueprints/Enum/E_Gender` (`KismetMathLibrary.Conv_IntToByte` (`KismetMathLibrary.RandomIntegerInRange` 0 (- (enumcount `/Game/Blueprints/Enum/E_Gender`) 1))))))
  (switch `/Game/Blueprints/Enum/E_Gender` _output_get_2
    (:`NewEnumerator2`
      (bind _name (`self.SetPersonName` "/Game/Blueprints/DataTable/DT_PersonNameCollection.DT_PersonNameCollection" "MaleName"))
      (set `local.Name` _name))
    (:`NewEnumerator1`
      (bind _name_2 (`self.SetPersonName` "/Game/Blueprints/DataTable/DT_PersonNameCollection.DT_PersonNameCollection" "FemaleName"))
      (set `local.Name` _name_2)))
  (bind _lastname (`self.SetPersonLastName`))
  (set `local.LastName` _lastname)
  (setmembers `/Game/Blueprints/Structure/F_PersonDetail` :`StructRef` (`self.Details`) :`Name` (`local.Name`) :`LastName` (`local.LastName`) :`Gender` (`local.Gender`) :`Age` (`local.Age`) :`AgeGroup` (`local.AgeGroup`) :`Task` "NewEnumerator9" :`ProfileAvatar` (select `/Game/Blueprints/Enum/E_Gender` (`local.Gender`) :`NewEnumerator2` "/Game/Texture/UI/Person/UI_Icon_Male.UI_Icon_Male" :`NewEnumerator1` "/Game/Texture/UI/Person/UI_Icon_Female.UI_Icon_Female" :!type "Texture2D Object Reference"))
  (`self.SetMesh`))

(fn `SetSpawnPoint`
  (bind _outactors (`GameplayStatics.GetAllActorsOfClass` "/Game/Blueprints/Components/Spawn/BP_SpawnPoint.BP_SpawnPoint_C"))
  (set `self.Spawn` (cast `/Game/Blueprints/Components/Spawn/BP_SpawnPoint` (`.ReturnValue` (`GameplayStatics.FindNearestActor` (`self.K2_GetActorLocation`) _outactors)) :!pure true)))

(fn `UpdateInventoryWidget`
  (bind _returnvalue (`WidgetComponent.GetWidget` (`self.PersonInfo`)))
  (`/Engine/EditorBlueprintResources/StandardMacros.IsValid` _returnvalue
    (:`Is Valid`
      (`/Game/Blueprints/UI/Person/WBP_PersonInfo.UpdatePersonInventory` (cast `/Game/Blueprints/UI/Person/WBP_PersonInfo` _returnvalue :!pure true)))))

(fn `UpdatePersonStats`
  (params (Waste :type "/Game/Blueprints/Actors/Waste/BP_Waste Object Reference"))
  (returns (StatsToExportParam :type "/Game/Blueprints/Structure/F_OverallInfo Structure"))
  (locals (Stats :type "/Game/Blueprints/Structure/F_Stats Structure") (Info :type "/Game/Blueprints/Structure/F_OverallInfo Structure"))
  (bind _stats (`self.Stats`))
  (bind _stats_2 (`self.Stats`))
  (bind _stats_3 (`self.Stats`))
  (bind ((`TotalOrganicWasteWeight_55_CD97D9E1488499C669AE47BA1609289A` _totalorganicwasteweight) (`TotalWeightGenerated_62_D278A50F44EDFB5F8BA78A9C3AC53A69` _totalweightgenerated)) (break `/Game/Blueprints/Structure/F_Stats` _stats))
  (bind ((`TotalWasteWeigh_57_BE5538EF4582794FEDE90095D7763206` _totalwasteweigh) (`TotalWeightGenerated_62_D278A50F44EDFB5F8BA78A9C3AC53A69` _totalweightgenerated_2)) (break `/Game/Blueprints/Structure/F_Stats` _stats_2))
  (bind ((`TotalRecyclableWasteWeight_56_BE899F404B2463B50D1250AE1D050569` _totalrecyclablewasteweight) (`TotalRecyclablePrice_59_54B91AE04B89188609D6DD9B937430ED` _totalrecyclableprice) (`TotalWeightGenerated_62_D278A50F44EDFB5F8BA78A9C3AC53A69` _totalweightgenerated_3)) (break `/Game/Blueprints/Structure/F_Stats` _stats_3))
  (bind ((`Name_34_90C7E46B4048F4C6621C8F87493905A4` _name) (`Description_35_FA3A56E8438BCBBAD3D3F19E2BF0C5A9` _description) (`Weight_6_CCA021244E9F8E30E0D2C282BDA939AC` _weight) (`Price_18_2B5D253C42D90CED3CEA0485A9C32E50` _price) (`Type_12_E4B9AF6E4BFB737C2F9D1DA63FAC2614` _type)) (break `/Game/Blueprints/Structure/F_WasteDetail` (`/Game/Blueprints/Actors/Waste/BP_Waste.Details` (`local.Waste`))))
  (`|ExecutionSequence`
    (:`then_0`
      (if (`KismetSystemLibrary.IsValid` (`local.Waste`))
        (switch `/Game/Blueprints/Enum/E_WasteType` _type
          (:`NewEnumerator0`
            ;[1 1 1] Organic Waste Stats
            (setmembers `/Game/Blueprints/Structure/F_Stats` :`StructRef` _stats :`TotalOrganicWasteWeight` (+ _totalorganicwasteweight _weight) :`TotalWeightGenerated` (+ _totalweightgenerated _weight))
            (setmembers `/Game/Blueprints/Structure/F_OverallInfo` :`StructRef` (`local.Info`) :`TotalOrganicWasteWeight` _weight :`TotalWeightGenerated` _weight))
          (:`NewEnumerator1`
            ;[1 1 1] Recyclable Waste Stats
            (setmembers `/Game/Blueprints/Structure/F_Stats` :`StructRef` _stats_3 :`TotalRecyclableWasteWeight` (+ _totalrecyclablewasteweight _weight) :`TotalRecyclablePrice` (+ _totalrecyclableprice _price) :`TotalWeightGenerated` (+ _totalweightgenerated_3 _weight) :!label _label)
            (setmembers `/Game/Blueprints/Structure/F_OverallInfo` :`StructRef` (`local.Info`) :`TotalRecyclableWasteWeight` _weight :`TotalRecyclablePrice` _price :`TotalWeightGenerated` _weight))
          (:`NewEnumerator2`
            (goto _label))
          (:`NewEnumerator3`
            (goto _label))
          (:`NewEnumerator4`
            (goto _label))
          (:`NewEnumerator7`
            (goto _label))
          (:`NewEnumerator8`
            ;[1 1 1] Waste Stats
            (setmembers `/Game/Blueprints/Structure/F_Stats` :`StructRef` _stats_2 :`TotalWasteWeigh` (+ _totalwasteweigh _weight) :`TotalWeightGenerated` (+ _totalweightgenerated_2 _weight))
            (setmembers `/Game/Blueprints/Structure/F_OverallInfo` :`StructRef` (`local.Info`) :`TotalWasteWeigh` _totalwasteweigh :`TotalWeightGenerated` _totalwasteweigh)))))
    (:`then_1`
      (return (`local.Info`)))))

(fn `UpdatePersonStatus`
  (params (NewParam :type "/Game/Blueprints/Enum/E_PersonStatus Enum" :default "NewEnumerator0"))
  (setmembers `/Game/Blueprints/Structure/F_PersonDetail` :`StructRef` (`self.Details`) :`Task` NewParam))

(fn `UserConstructionScript`)