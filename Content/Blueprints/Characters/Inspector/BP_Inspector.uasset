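; Inspector service character, a child of a shared person class, that runs BT_Inspector for a timed duration read from DT_Services.
; BeginPlay disables engine lifespan, maxes conscience and mood, and caches the game state and time widget.
; A one-second timer counts Lifespan down while DecreaseLifespan is set and refreshes that widget, without destroying the actor itself.
; On destruction it decrements the active inspector count in the game state.
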(event `self.ReceiveBeginPlay`
  ;[1 1 1] Event BeginPlay
  (`parent.ReceiveBeginPlay`)
  (`self.SetLifeSpan` 0.0)
  (bind _returnvalue (`|GetDataTableRow` "/Game/Blueprints/DataTable/DT_Services.DT_Services" "Inspector")
    (:`then`
      (bind ((`Duration_11_F3B0E8F94D2078569F9CE5B3D227ED6E` _duration)) (break `/Game/Blueprints/Structure/F_Service` _returnvalue))
      (set `self.Lifespan` _duration)
      (set `self.MaxLifespan` _duration)
      (`AIController.RunBehaviorTree` (`AIBlueprintHelperLibrary.GetAIController` self) "/Game/Blueprints/AI/Inspector/BT_Inspector.BT_Inspector")
      (`self.SetPersonDetails`)
      (bind _asbp_game_state (cast `/Game/Blueprints/Game/BP_GameState` (`GameplayStatics.GetGameState`)))
      (bind _output_get (set `self.GameState` _asbp_game_state))
      (`/Game/Blueprints/Game/BP_GameState.UpdateOverallInfo` _output_get (make `/Game/Blueprints/Structure/F_OverallInfo` :`TotalHiredInspectors` 1 :`TotalActiveInspectors` 1))
      (bind _aswbp_person_icon (cast `/Game/Blueprints/UI/Person/WBP_PersonIcon` (`WidgetComponent.GetWidget` (`self.TimeWidget`))))
      (bind _output_get_2 (set `self.WBP_TimeWidge` _aswbp_person_icon))
      (`/Game/Blueprints/UI/Person/WBP_PersonIcon.Set Time` _output_get_2 (`self.Lifespan`) (`self.MaxLifespan`))
      (`KismetSystemLibrary.K2_SetTimer` null "UpdateLifespan" 1.0 true))))

(event `UpdateLifespan`
  (bind _lifespan (`self.Lifespan`))
  ;[1 1 1] Event BeginPlay
  (if (`self.bDecreaseLifespan`)
    (bind _output_get (set `self.Lifespan` (`KismetMathLibrary.FClamp` (- _lifespan 1.0) 0.0 _lifespan)))
    (`/Game/Blueprints/UI/Person/WBP_PersonIcon.Set Time` (`self.WBP_TimeWidge`) _output_get (`self.MaxLifespan`))))

(event `self.ReceiveDestroyed`
  ;[1 1 1] Event Destoyed
  (`/Game/Blueprints/Game/BP_GameState.UpdateOverallInfo` (`self.GameState`) (make `/Game/Blueprints/Structure/F_OverallInfo` :`TotalActiveInspectors` -1)))

(fn `SetPersonDetails`
  (`parent.SetPersonDetails`)
  (setmembers `/Game/Blueprints/Structure/F_PersonDetail` :`StructRef` (`self.Details`) :`Conscience` 100.0 :`Mood` 100.0))

(fn `UserConstructionScript`
  (`parent.UserConstructionScript`))