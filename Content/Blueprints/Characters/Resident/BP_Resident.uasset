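; BP_Resident is a resident AI character that periodically generates waste and feeds awareness and mood into the game's overall totals.
; On BeginPlay it starts the BT_Resident behavior tree, randomizes starting Conscience and Mood, and reports both to BP_GameState.
; A looping timer with a per-resident random interval calls Generate Waste, which defers to the parent class, as does the tail of SetPersonDetails.
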(event `self.ReceiveBeginPlay`
  (bind ((`Conscience_35_519E32E14799A62A65B328B0DD622DAE` _conscience) (`Mood_36_7BCD7D5140C9C277061647BB3AC58066` _mood)) (break `/Game/Blueprints/Structure/F_PersonDetail` (`self.Details`)))
  (`parent.ReceiveBeginPlay`)
  (bind _asbp_game_state (cast `/Game/Blueprints/Game/BP_GameState` (`GameplayStatics.GetGameState`)))
  (set `self.GameState` _asbp_game_state)
  (`AIController.RunBehaviorTree` (`AIBlueprintHelperLibrary.GetAIController` (`self.GetController`)) "/Game/Blueprints/AI/Resident/BT_Resident.BT_Resident")
  (`self.SetPersonDetails`)
  (`KismetSystemLibrary.K2_SetTimer` null "Generate Waste" (`KismetMathLibrary.RandomFloatInRange` 30.0 45.0) true 20.0)
  (`/Game/Blueprints/Game/BP_GameState.UpdateOverallInfo` (`self.GameState`) (make `/Game/Blueprints/Structure/F_OverallInfo` :`TotalAwarenessPoints` _conscience :`TotalMoodPoints` _mood)))

(fn `Generate Waste`
  (`parent.Generate Waste`))

(fn `SetPersonDetails`
  (setmembers `/Game/Blueprints/Structure/F_PersonDetail` :`StructRef` (`self.Details`) :`Conscience` (`KismetMathLibrary.RandomFloatInRange` 20.0 35.0) :`Mood` (`KismetMathLibrary.RandomFloatInRange` 30.0 45.0))
  (`parent.SetPersonDetails`))

(fn `UserConstructionScript`
  (`parent.UserConstructionScript`))