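; BP_Pedestrian is a pedestrian character that generates waste as it runs the BT_Pedestrian behavior tree.
; On BeginPlay it caches the game state, starts the tree, sets person details and spawn point, and starts a looping, randomly timed waste timer.
; It extends parent functions, randomizing Conscience and Mood and generating waste only while total generated weight is within a small threshold, re-rolled on each call.
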(event `self.ReceiveBeginPlay`
  (bind _asbp_game_state (cast `/Game/Blueprints/Game/BP_GameState` (`GameplayStatics.GetGameState`)))
  (set `self.GameState` _asbp_game_state)
  (`AIController.RunBehaviorTree` (`AIBlueprintHelperLibrary.GetAIController` self) "/Game/Blueprints/AI/Pedestrian/BT_Pedestrian.BT_Pedestrian")
  (`self.SetPersonDetails`)
  (`self.SetSpawnPoint`)
  (`KismetSystemLibrary.K2_SetTimer` null "Generate Waste" (`KismetMathLibrary.RandomFloatInRange` 10.0 20.0) true))

(fn `Generate Waste`
  (if (<= (`.TotalWeightGenerated_62_D278A50F44EDFB5F8BA78A9C3AC53A69` (break `/Game/Blueprints/Structure/F_Stats` (`self.Stats`))) (`KismetMathLibrary.RandomFloatInRange` 0.5 1.0))
    (`parent.Generate Waste`)))

(fn `SetPersonDetails`
  (bind _returnvalue (`KismetMathLibrary.RandomFloatInRange` 10.0 100.0))
  (`parent.SetPersonDetails`)
  (setmembers `/Game/Blueprints/Structure/F_PersonDetail` :`StructRef` (`self.Details`) :`Conscience` _returnvalue :`Mood` _returnvalue))

(fn `UserConstructionScript`
  (`parent.UserConstructionScript`))